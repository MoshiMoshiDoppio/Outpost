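; Laser knife weapon that attaches to the player's weapon socket on spawn and plays a knife hold montage.
; Left and right click play different stab montages, each setting its own damage multiplier and scaling play rate with the player's clamped fire rate.
; A cooldown flag and weapon swapping block attacks; each stab's montage notify restores the hold pose and clears the cooldown.
; Damage application is not handled in this graph.
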(event EventBeginPlay
  (|CallParentFunction)
  (Variables|Default|SetAmmo 1)
  (bind _asplayer_character_bp (Utilities|Casting|CastToPlayerCharacterBP (Game|GetPlayerCharacter 0)))
  (Variables|Default|SetAs%20Player%20Character%20BP _asplayer_character_bp)
  (Animation|Montage|PlayMontage (Variables|/Script/Engine.Character|GetMesh _asplayer_character_bp) "/Game/Models/Player/Animations/PlayerHoldKnife_Montage.PlayerHoldKnife_Montage"
    (:then
      (Transformation|AttachComponentToComponent (Variables|/Script/Engine.Character|GetMesh _asplayer_character_bp) "WeaponSocket" "SnapToTarget" "KeepRelative" "KeepWorld" true))))

(event Collision|EventActorBeginOverlap
  (params (OtherActor :type Actor%20Object%20Reference))
  (|CallParentFunction OtherActor) ; This node is disabled and will not be called.\nDrag off pins to build functionality.
)

(event EventTick
  (params (DeltaSeconds :type Float%20%28single-precision%29))
  (|CallParentFunction DeltaSeconds) ; This node is disabled and will not be called.\nDrag off pins to build functionality.
)

(event EventLeftClick
  (bind _as_player_character_bp (Variables|Default|GetAs%20Player%20Character%20BP))
  (bind _mesh (Variables|/Script/Engine.Character|GetMesh _as_player_character_bp))
  (if (and (not (Variables|Default|GetFireCD)) (not (Variables|/Game/Blueprints/Player/PlayerCharacterBP.PlayerCharacterBP_C|GetSwappingWeapons (Variables|Default|GetAs%20Player%20Character%20BP))))
    (Variables|Default|SetFireCD true)
    (Animation|Montage|PlayMontage _mesh "/Game/Models/Player/Animations/KnifeStab1_Montage.KnifeStab1_Montage" (Math|Float|Clamp(Float) (+ (Variables|/Game/Blueprints/Player/PlayerCharacterBP.PlayerCharacterBP_C|GetFireRate _as_player_character_bp) 1.0) 1.0 1.5)
      (:then
        (Variables|Default|SetDamageX 1.5))
      (:OnNotifyBegin
        (Animation|Montage|PlayMontage _mesh "/Game/Models/Player/Animations/PlayerHoldKnife_Montage.PlayerHoldKnife_Montage"
          (:then
            (Variables|Default|SetFireCD false)))))))

(event EventRightClick
  (bind _as_player_character_bp (Variables|Default|GetAs%20Player%20Character%20BP))
  (bind _mesh (Variables|/Script/Engine.Character|GetMesh _as_player_character_bp))
  (if (and (not (Variables|Default|GetFireCD)) (not (Variables|/Game/Blueprints/Player/PlayerCharacterBP.PlayerCharacterBP_C|GetSwappingWeapons (Variables|Default|GetAs%20Player%20Character%20BP))))
    (Variables|Default|SetFireCD true)
    (Animation|Montage|PlayMontage _mesh "/Game/Models/Player/Animations/KnifeStab2_Montage.KnifeStab2_Montage" (Math|Float|Clamp(Float) (+ (Variables|/Game/Blueprints/Player/PlayerCharacterBP.PlayerCharacterBP_C|GetFireRate _as_player_character_bp) 1.0) 1.0 1.25)
      (:then
        (Variables|Default|SetDamageX 0.8))
      (:OnNotifyBegin
        (Animation|Montage|PlayMontage _mesh "/Game/Models/Player/Animations/PlayerHoldKnife_Montage.PlayerHoldKnife_Montage"
          (:then
            (Variables|Default|SetFireCD false)))))))

(fn ConstructionScript
  (|CallParentFunction))