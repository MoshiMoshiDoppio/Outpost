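; Player pistol-style build gun that attaches to the character's weapon socket and places, previews and removes building blocks.
; Left click line-traces along camera forward to spawn the selected block; scroll rotates pitch or yaw, right and middle click cycle type and material.
; GhostBlock previews placement by respawning a short-lived, collision-free block on a timer.
; Reload destroys the targeted block, or every placed block when none is hit.
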(event Custom|GhostBlock
  (bind _firepoint (Variables|Default|GetFirePoint))
  (bind _returnvalue (Transformation|GetWorldLocation _firepoint))
  (Utilities|Time|SetTimerbyEvent (delegate Custom|GhostBlock) 0.1 true)
  (bind (_outhit _returnvalue_2) (Collision|LineTraceByChannel _returnvalue (+ _returnvalue (* (Math|Vector|GetForwardVector (Variables|/Game/Blueprints/Player/PlayerCharacterBP.PlayerCharacterBP_C|GetFollowCamera (Variables|Default|GetAs%20Player%20Character%20BP))) 1e+03)) "TraceTypeQuery2" false 0 "None"))
  (if _returnvalue_2
    (bind _returnvalue_3 (Game|SpawnActorfromClass (Utilities|Array|Get(acopy) (Variables|Default|GetBlockTypes) (Variables|Default|GetBlockType)) (Math|Transform|MakeTransform (.Location (Collision|BreakHitResult _outhit)) (Math|Rotator|MakeRotator 0.0 (Variables|Default|GetBlockY) (Variables|Default|GetBlockZ)) "1.000000,1.000000,1.000000") "Undefined" "MultiplyWithRoot" 0 0))
    (Rendering|Material|SetMaterial (Variables|/Game/Blueprints/BuildingBlocks/BuildBlockParentBP.BuildBlockParentBP_C|GetBlockMesh _returnvalue_3) 0 (Utilities|Array|Get(acopy) (Variables|Default|GetGhostBlockMats) (Variables|Default|GetBlockMatIndex)))
    (Collision|SetCollisionEnabled (Variables|/Game/Blueprints/BuildingBlocks/BuildBlockParentBP.BuildBlockParentBP_C|GetBlockMesh _returnvalue_3) "NoCollision")
    (Utilities|FlowControl|Delay 0.1)
    (Actor|DestroyActor _returnvalue_3)))

(event EventBeginPlay
  (|CallParentFunction)
  (bind _asplayer_character_bp (Utilities|Casting|CastToPlayerCharacterBP (Game|GetPlayerCharacter 0)))
  (Variables|Default|SetAs%20Player%20Character%20BP _asplayer_character_bp)
  (Animation|Montage|PlayMontage (Variables|/Script/Engine.Character|GetMesh _asplayer_character_bp) "/Game/Models/Player/Animations/PlayerHoldPistol_Montage.PlayerHoldPistol_Montage"
    (:then
      (Transformation|AttachComponentToComponent (Variables|/Script/Engine.Character|GetMesh _asplayer_character_bp) "WeaponSocket" "SnapToTarget" "KeepRelative" "KeepWorld" true)
      (CallFunction|GhostBlock))))

(event Collision|EventActorBeginOverlap
  (params (OtherActor :type Actor%20Object%20Reference))
  (|CallParentFunction OtherActor) ; This node is disabled and will not be called.\nDrag off pins to build functionality.
)

(event EventTick
  (params (DeltaSeconds :type Float%20%28single-precision%29))
  (|CallParentFunction DeltaSeconds) ; This node is disabled and will not be called.\nDrag off pins to build functionality.
)

(event EventLeftClick
  (bind _as_player_character_bp (Variables|Default|GetAs%20Player%20Character%20BP))
  (bind _firepoint (Variables|Default|GetFirePoint))
  (bind _returnvalue (Transformation|GetWorldLocation _firepoint))
  (bind _mesh (Variables|/Script/Engine.Character|GetMesh _as_player_character_bp))
  (if (and (not (Variables|Default|GetFireCD)) (not (Variables|/Game/Blueprints/Player/PlayerCharacterBP.PlayerCharacterBP_C|GetSwappingWeapons (Variables|Default|GetAs%20Player%20Character%20BP))))
    (Variables|Default|SetFireCD true)
    (Animation|Montage|PlayMontage _mesh "/Game/Models/Player/Animations/PlayerPistolFire_Montage.PlayerPistolFire_Montage" 2.0
      (:then
        (bind (_outhit _returnvalue_2) (Collision|LineTraceByChannel _returnvalue (+ _returnvalue (* (Math|Vector|GetForwardVector (Variables|/Game/Blueprints/Player/PlayerCharacterBP.PlayerCharacterBP_C|GetFollowCamera (Variables|Default|GetAs%20Player%20Character%20BP))) 1e+03)) "TraceTypeQuery2" false 0 "None"))
        (if _returnvalue_2
          (bind _returnvalue_3 (Game|SpawnActorfromClass (Utilities|Array|Get(acopy) (Variables|Default|GetBlockTypes) (Variables|Default|GetBlockType)) (Math|Transform|MakeTransform (.Location (Collision|BreakHitResult _outhit)) (Math|Rotator|MakeRotator 0.0 (Variables|Default|GetBlockY) (Variables|Default|GetBlockZ)) "1.000000,1.000000,1.000000") "Undefined" "MultiplyWithRoot" 0 0))
          (Rendering|Material|SetMaterial (Variables|/Game/Blueprints/BuildingBlocks/BuildBlockParentBP.BuildBlockParentBP_C|GetBlockMesh _returnvalue_3) 0 (Utilities|Array|Get(acopy) (Variables|Default|GetBlockMats) (Variables|Default|GetBlockMatIndex)))
          (Rendering|SetVisibility (Variables|/Game/Blueprints/BuildingBlocks/BuildBlockCubeBP.BuildBlockCubeBP_C|GetArrow _returnvalue_3) false false)
          (Variables|/Game/Blueprints/BuildingBlocks/BuildBlockParentBP.BuildBlockParentBP_C|SetGhost _returnvalue_3 false)))
      (:OnNotifyBegin
        (Animation|Montage|PlayMontage _mesh "/Game/Models/Player/Animations/PlayerHoldPistol_Montage.PlayerHoldPistol_Montage"
          (:then
            (Variables|Default|SetFireCD false)))))))

(event EventReload
  (bind _firepoint (Variables|Default|GetFirePoint))
  (bind _returnvalue (Transformation|GetWorldLocation _firepoint))
  (Utilities|FlowControl|DoOnce false :!label _label
    (:Completed
      (bind _outhit (Collision|LineTraceByChannel _returnvalue (+ _returnvalue (* (Math|Vector|GetForwardVector (Variables|/Game/Blueprints/Player/PlayerCharacterBP.PlayerCharacterBP_C|GetFollowCamera (Variables|Default|GetAs%20Player%20Character%20BP))) 3.5e+03)) "TraceTypeQuery2" false 0 "None"))
      (bind _asbuild_block_parent_bp (Utilities|Casting|CastToBuildBlockParentBP (.HitActor (Collision|BreakHitResult _outhit)))
        (:then
          (Actor|DestroyActor _asbuild_block_parent_bp)
          (Utilities|FlowControl|Delay 0.5)
          (goto _label Reset))
        (:CastFailed
          (bind _outactors (Actor|GetAllActorsOfClass "/Game/Blueprints/BuildingBlocks/BuildBlockParentBP.BuildBlockParentBP_C"))
          (if (> (Utilities|Array|Length _outactors) 0)
            (for _array_element _outactors
              (if (not (Variables|/Game/Blueprints/BuildingBlocks/BuildBlockParentBP.BuildBlockParentBP_C|GetGhost _array_element))
                (Actor|DestroyActor _array_element)))
            (Utilities|FlowControl|Delay 0.5)
            (goto _label Reset)))))))

(event EventScrollDown
  ;[1 1 1] Scroll
  (if (>= (+ (Variables|Default|GetBlockZ) 9e+01) 3.6e+02)
    (Variables|Default|SetBlockZ 0.0)
    (else
      (Variables|Default|SetBlockZ (+ (Variables|Default|GetBlockZ) 9e+01)))))

(event EventScrollUp
  ;[1 1 1] Scroll
  (if (>= (+ (Variables|Default|GetBlockY) 9e+01) 3.6e+02)
    (Variables|Default|SetBlockY 0.0)
    (else
      (Variables|Default|SetBlockY (+ (Variables|Default|GetBlockY) 9e+01)))))

(event EventRightClick
  ;[1 1 1] Right Click
  (if (>= (+ (Variables|Default|GetBlockType) 1) (Utilities|Array|Length (Variables|Default|GetBlockTypes)))
    (Variables|Default|SetBlockType 0)
    (else
      (Variables|Default|SetBlockType (+ (Variables|Default|GetBlockType) 1)))))

(event EventMiddleClick
  ;[1 1 1] Middle Click
  (if (>= (+ (Variables|Default|GetBlockMatIndex) 1) (Utilities|Array|Length (Variables|Default|GetBlockMats)))
    (Variables|Default|SetBlockMatIndex 0)
    (else
      (Variables|Default|SetBlockMatIndex (+ (Variables|Default|GetBlockMatIndex) 1)))))

(fn ConstructionScript
  (|CallParentFunction))