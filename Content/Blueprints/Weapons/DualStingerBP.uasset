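; Dual Stinger player weapon: two socket-attached pistols with separate ammo counters and an on-screen ammo widget.
; Left and right click fire each gun, scrolling fires both, with montage notifies clearing the fire cooldown.
; Shots are camera-directed line traces that damage enemies and show damage widgets, scaled by player stats and the Overcharge upgrade.
; Empty guns or manual reload enter a shared DoOnce that refills both magazines.
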(event EventBeginPlay
  (|CallParentFunction)
  (bind _asoagame_instance (Utilities|Casting|CastToOAGameInstance (Game|GetGameInstance)))
  (if (Utilities|Array|ContainsItem (Variables|/Game/Blueprints/GamemodeInstance/OAGameInstance.OAGameInstance_C|GetPlayerWeaponUpgrades _asoagame_instance) "Overcharge")
    (Variables|Default|SetOCDamage 50))
  (bind _asplayer_character_bp (Utilities|Casting|CastToPlayerCharacterBP (Game|GetPlayerCharacter 0)))
  (Variables|Default|SetAmmo (+ (Variables|/Game/Blueprints/Player/PlayerCharacterBP.PlayerCharacterBP_C|GetAmmo _asplayer_character_bp) 20))
  (Variables|Default|SetAmmo2 (+ (Variables|/Game/Blueprints/Player/PlayerCharacterBP.PlayerCharacterBP_C|GetAmmo _asplayer_character_bp) 20))
  (Variables|Default|SetAs%20Player%20Character%20BP _asplayer_character_bp)
  (Animation|Montage|PlayMontage (Variables|/Script/Engine.Character|GetMesh _asplayer_character_bp) "/Game/Models/Player/Animations/PlayerDualPistolHold_Montage.PlayerDualPistolHold_Montage"
    (:then
      (Transformation|AttachComponentToComponent (Variables|/Script/Engine.Character|GetMesh _asplayer_character_bp) "WeaponSocket" "SnapToTarget" "KeepRelative" "KeepWorld" true)
      (Transformation|AttachComponentToComponent (Variables|Default|GetGun2) (Variables|/Script/Engine.Character|GetMesh _asplayer_character_bp) "WeaponSocket2" "SnapToTarget" "KeepRelative" "KeepWorld" true)
      (bind _returnvalue (UserInterface|CreateWidget "/Game/Widgets/Ammo/DualStingerAmmoWidget.DualStingerAmmoWidget_C"))
      (UserInterface|Viewport|AddtoViewport _returnvalue 0))))

(event EventRemoveWidget
  (Widget|RemovefromParent (stale EventBeginPlay _returnvalue)))

(event EventLeftClick
  (bind _as_player_character_bp (Variables|Default|GetAs%20Player%20Character%20BP))
  (bind _firepoint (Variables|Default|GetFirePoint))
  (bind _as_player_character_bp_2 (Variables|Default|GetAs%20Player%20Character%20BP))
  (bind _as_player_character_bp_3 (Variables|Default|GetAs%20Player%20Character%20BP))
  (bind _as_player_character_bp_4 (Variables|Default|GetAs%20Player%20Character%20BP))
  (bind _as_player_character_bp_5 (Variables|Default|GetAs%20Player%20Character%20BP))
  (bind _as_player_character_bp_6 (Variables|Default|GetAs%20Player%20Character%20BP))
  (bind _firepoint_2 (Variables|Default|GetFirePoint))
  (bind _ocdamage (Variables|Default|GetOCDamage))
  (bind _returnvalue (Transformation|GetWorldLocation _firepoint))
  (bind _damage (Variables|/Game/Blueprints/Player/PlayerCharacterBP.PlayerCharacterBP_C|GetDamage _as_player_character_bp_6))
  (bind _mesh (Variables|/Script/Engine.Character|GetMesh _as_player_character_bp_4))
  (bind _mesh_2 (Variables|/Script/Engine.Character|GetMesh _as_player_character_bp))
  (bind _returnvalue_2 (+ _damage 25 _ocdamage))
  (if (> (Variables|Default|GetAmmo) 0)
    (if (Math|Boolean|ANDBoolean (not (Variables|Default|GetFireCD)) (not (Variables|Default|GetReload?)) (not (Variables|/Game/Blueprints/Player/PlayerCharacterBP.PlayerCharacterBP_C|GetSwappingWeapons (Variables|Default|GetAs%20Player%20Character%20BP))))
      (Variables|Default|SetFireCD true)
      (Animation|Montage|PlayMontage _mesh "/Game/Models/Player/Animations/PlayerDualPistolFireL_Montage.PlayerDualPistolFireL_Montage" (+ (Variables|/Game/Blueprints/Player/PlayerCharacterBP.PlayerCharacterBP_C|GetFireRate _as_player_character_bp_4) 1.65)
        (:then
          (bind _result (Math|Integer|DecrementInt (Variables|Default|GetAmmo))
            (:%20%20
              (Utilities|Array|SetArrayElem (Variables|/Game/Blueprints/Player/PlayerCharacterBP.PlayerCharacterBP_C|GetWeaponAmmo _as_player_character_bp_3) (Variables|/Game/Blueprints/Player/PlayerCharacterBP.PlayerCharacterBP_C|GetWeaponSlot _as_player_character_bp_3) _result)
              (bind _returnvalue_3 (Game|SpawnActorfromClass "/Game/Blueprints/FX/MuzzleFlash/StingerMuzzleFlashBP.StingerMuzzleFlashBP_C" (Transformation|GetWorldTransform _firepoint_2) "Undefined" "MultiplyWithRoot" 0 0))
              (Transformation|AttachComponentToComponent _returnvalue_3 _firepoint_2 "None" "SnapToTarget" "SnapToTarget" "SnapToTarget" true)
              (bind _outhit (Collision|LineTraceByChannel _returnvalue (+ _returnvalue (* (Math|Vector|GetForwardVector (Variables|/Game/Blueprints/Player/PlayerCharacterBP.PlayerCharacterBP_C|GetFollowCamera _as_player_character_bp_2)) (+ 8e+03 (Variables|/Game/Blueprints/Player/PlayerCharacterBP.PlayerCharacterBP_C|GetFireRange _as_player_character_bp_2)))) "TraceTypeQuery2" false 0 "None"))
              (bind _asenemy_parent_bp (Utilities|Casting|CastToEnemyParentBP (.HitActor (Collision|BreakHitResult _outhit))))
              (Default|TakeDamage _asenemy_parent_bp _returnvalue_2)
              (bind _returnvalue_4 (UserInterface|CreateWidget "/Game/Widgets/Hud/DamageWidget.DamageWidget_C" 0 _returnvalue_2))
              (UserInterface|Viewport|AddtoViewport _returnvalue_4 0))))
        (:OnNotifyBegin
          (if (== _result 0)
            (Utilities|FlowControl|DoOnce false :!label _label
              (:Completed
                (Variables|Default|SetReload? true)
                (Animation|Montage|PlayMontage _mesh_2 "/Game/Models/Player/Animations/PlayerReloadPistolBoth_Montage.PlayerReloadPistolBoth_Montage" (+ (Variables|/Game/Blueprints/Player/PlayerCharacterBP.PlayerCharacterBP_C|GetReloadSpeed (Variables|Default|GetAs%20Player%20Character%20BP)) 1.0)
                  (:OnNotifyBegin
                    (Animation|Montage|PlayMontage _mesh_2 "/Game/Models/Player/Animations/PlayerDualPistolHold_Montage.PlayerDualPistolHold_Montage"
                      (:then
                        (bind _output_get (Variables|Default|SetAmmo (+ (Variables|/Game/Blueprints/Player/PlayerCharacterBP.PlayerCharacterBP_C|GetAmmo _as_player_character_bp_5) 20)))
                        (Variables|Default|SetAmmo2 (+ (Variables|/Game/Blueprints/Player/PlayerCharacterBP.PlayerCharacterBP_C|GetAmmo _as_player_character_bp_5) 20))
                        (Utilities|Array|SetArrayElem (Variables|/Game/Blueprints/Player/PlayerCharacterBP.PlayerCharacterBP_C|GetWeaponAmmo _as_player_character_bp_5) (Variables|/Game/Blueprints/Player/PlayerCharacterBP.PlayerCharacterBP_C|GetWeaponSlot _as_player_character_bp_5) _output_get)
                        (Utilities|FlowControl|Delay 0.2)
                        (Variables|Default|SetReload? false)
                        (Variables|Default|SetFireCD false)
                        (goto _label Reset)))))))
            (else
              (Animation|Montage|PlayMontage _mesh "/Game/Models/Player/Animations/PlayerDualPistolHold_Montage.PlayerDualPistolHold_Montage"
                (:then
                  (Variables|Default|SetFireCD false))))))))
    (else
      (goto _label))))

(event EventRightClick
  (bind _as_player_character_bp (Variables|Default|GetAs%20Player%20Character%20BP))
  (bind _as_player_character_bp_2 (Variables|Default|GetAs%20Player%20Character%20BP))
  (bind _as_player_character_bp_3 (Variables|Default|GetAs%20Player%20Character%20BP))
  (bind _firepoint2 (Variables|Default|GetFirePoint2))
  (bind _as_player_character_bp_4 (Variables|Default|GetAs%20Player%20Character%20BP))
  (bind _as_player_character_bp_5 (Variables|Default|GetAs%20Player%20Character%20BP))
  (bind _firepoint2_2 (Variables|Default|GetFirePoint2))
  (bind _ocdamage (Variables|Default|GetOCDamage))
  (bind _returnvalue (Transformation|GetWorldLocation _firepoint2))
  (bind _damage (Variables|/Game/Blueprints/Player/PlayerCharacterBP.PlayerCharacterBP_C|GetDamage _as_player_character_bp_2))
  (bind _mesh (Variables|/Script/Engine.Character|GetMesh _as_player_character_bp))
  (bind _returnvalue_2 (+ _damage 25 _ocdamage))
  (if (> (Variables|Default|GetAmmo2) 0)
    (if (Math|Boolean|ANDBoolean (not (Variables|Default|GetFireCD)) (not (Variables|Default|GetReload?)) (not (Variables|/Game/Blueprints/Player/PlayerCharacterBP.PlayerCharacterBP_C|GetSwappingWeapons (Variables|Default|GetAs%20Player%20Character%20BP))))
      (Variables|Default|SetFireCD true)
      (Animation|Montage|PlayMontage _mesh "/Game/Models/Player/Animations/PlayerDualPistolFireR_Montage.PlayerDualPistolFireR_Montage" (+ (Variables|/Game/Blueprints/Player/PlayerCharacterBP.PlayerCharacterBP_C|GetFireRate (Variables|Default|GetAs%20Player%20Character%20BP)) 1.65)
        (:then
          (bind _result (Math|Integer|DecrementInt (Variables|Default|GetAmmo2))
            (:%20%20
              (Utilities|Array|SetArrayElem (Variables|/Game/Blueprints/Player/PlayerCharacterBP.PlayerCharacterBP_C|GetWeaponAmmo _as_player_character_bp_3) (Variables|/Game/Blueprints/Player/PlayerCharacterBP.PlayerCharacterBP_C|GetWeaponSlot _as_player_character_bp_3) _result)
              (bind _returnvalue_3 (Game|SpawnActorfromClass "/Game/Blueprints/FX/MuzzleFlash/StingerMuzzleFlashBP.StingerMuzzleFlashBP_C" (Transformation|GetWorldTransform _firepoint2_2) "Undefined" "MultiplyWithRoot" 0 0))
              (Transformation|AttachComponentToComponent _returnvalue_3 _firepoint2_2 "None" "SnapToTarget" "SnapToTarget" "SnapToTarget" true)
              (bind _outhit (Collision|LineTraceByChannel _returnvalue (+ _returnvalue (* (Math|Vector|GetForwardVector (Variables|/Game/Blueprints/Player/PlayerCharacterBP.PlayerCharacterBP_C|GetFollowCamera _as_player_character_bp_4)) (+ 8e+03 (Variables|/Game/Blueprints/Player/PlayerCharacterBP.PlayerCharacterBP_C|GetFireRange _as_player_character_bp_4)))) "TraceTypeQuery2" false 0 "None"))
              (bind _asenemy_parent_bp (Utilities|Casting|CastToEnemyParentBP (.HitActor (Collision|BreakHitResult _outhit))))
              (Default|TakeDamage _asenemy_parent_bp _returnvalue_2)
              (bind _returnvalue_4 (UserInterface|CreateWidget "/Game/Widgets/Hud/DamageWidget.DamageWidget_C" 0 _returnvalue_2))
              (UserInterface|Viewport|AddtoViewport _returnvalue_4 0))))
        (:OnNotifyBegin
          (if (== _result 0)
            (Utilities|FlowControl|DoOnce false :!label _label
              (:Completed
                (Variables|Default|SetReload? true)
                (Animation|Montage|PlayMontage _mesh "/Game/Models/Player/Animations/PlayerReloadPistolBoth_Montage.PlayerReloadPistolBoth_Montage" (+ (Variables|/Game/Blueprints/Player/PlayerCharacterBP.PlayerCharacterBP_C|GetReloadSpeed (Variables|Default|GetAs%20Player%20Character%20BP)) 1.0)
                  (:OnNotifyBegin
                    (Animation|Montage|PlayMontage _mesh "/Game/Models/Player/Animations/PlayerDualPistolHold_Montage.PlayerDualPistolHold_Montage"
                      (:then
                        (bind _output_get (Variables|Default|SetAmmo (+ (Variables|/Game/Blueprints/Player/PlayerCharacterBP.PlayerCharacterBP_C|GetAmmo _as_player_character_bp_5) 20)))
                        (Variables|Default|SetAmmo2 (+ (Variables|/Game/Blueprints/Player/PlayerCharacterBP.PlayerCharacterBP_C|GetAmmo _as_player_character_bp_5) 20))
                        (Utilities|Array|SetArrayElem (Variables|/Game/Blueprints/Player/PlayerCharacterBP.PlayerCharacterBP_C|GetWeaponAmmo _as_player_character_bp_5) (Variables|/Game/Blueprints/Player/PlayerCharacterBP.PlayerCharacterBP_C|GetWeaponSlot _as_player_character_bp_5) _output_get)
                        (Utilities|FlowControl|Delay 0.2)
                        (Variables|Default|SetReload? false)
                        (Variables|Default|SetFireCD false)
                        (goto _label Reset)))))))
            (else
              (Animation|Montage|PlayMontage (Variables|/Script/Engine.Character|GetMesh (Variables|Default|GetAs%20Player%20Character%20BP)) "/Game/Models/Player/Animations/PlayerDualPistolHold_Montage.PlayerDualPistolHold_Montage"
                (:then
                  (Variables|Default|SetFireCD false))))))))
    (else
      (goto _label))))

(event EventScrollUp
  (bind _as_player_character_bp (Variables|Default|GetAs%20Player%20Character%20BP))
  (bind _as_player_character_bp_2 (Variables|Default|GetAs%20Player%20Character%20BP))
  (bind _firepoint (Variables|Default|GetFirePoint))
  (bind _as_player_character_bp_3 (Variables|Default|GetAs%20Player%20Character%20BP))
  (bind _firepoint2 (Variables|Default|GetFirePoint2))
  (bind _as_player_character_bp_4 (Variables|Default|GetAs%20Player%20Character%20BP))
  (bind _as_player_character_bp_5 (Variables|Default|GetAs%20Player%20Character%20BP))
  (bind _as_player_character_bp_6 (Variables|Default|GetAs%20Player%20Character%20BP))
  (bind _as_player_character_bp_7 (Variables|Default|GetAs%20Player%20Character%20BP))
  (bind _firepoint2_2 (Variables|Default|GetFirePoint2))
  (bind _as_player_character_bp_8 (Variables|Default|GetAs%20Player%20Character%20BP))
  (bind _firepoint_2 (Variables|Default|GetFirePoint))
  (bind _ocdamage (Variables|Default|GetOCDamage))
  (bind _ocdamage_2 (Variables|Default|GetOCDamage))
  (bind _returnvalue (Transformation|GetWorldLocation _firepoint))
  (bind _returnvalue_2 (Transformation|GetWorldLocation _firepoint2))
  (bind _damage (Variables|/Game/Blueprints/Player/PlayerCharacterBP.PlayerCharacterBP_C|GetDamage _as_player_character_bp_2))
  (bind _damage_2 (Variables|/Game/Blueprints/Player/PlayerCharacterBP.PlayerCharacterBP_C|GetDamage _as_player_character_bp_8))
  (bind _mesh (Variables|/Script/Engine.Character|GetMesh _as_player_character_bp_5))
  (bind _mesh_2 (Variables|/Script/Engine.Character|GetMesh _as_player_character_bp))
  (bind _returnvalue_3 (+ _damage_2 25 _ocdamage))
  (bind _returnvalue_4 (+ _damage 25 _ocdamage_2))
  (if (and (not (Variables|Default|GetFireCD)) (not (Variables|Default|GetReload?)))
    (if (> (Variables|Default|GetAmmo) 0)
      (if (> (Variables|Default|GetAmmo2) 0)
        (Animation|Montage|PlayMontage _mesh "/Game/Models/Player/Animations/PlayerDualPistolFireBoth_Montage.PlayerDualPistolFireBoth_Montage" (+ (Variables|/Game/Blueprints/Player/PlayerCharacterBP.PlayerCharacterBP_C|GetFireRate (Variables|Default|GetAs%20Player%20Character%20BP)) 1.65)
          (:then
            (Variables|Default|SetFireCD true)
            (Math|Integer|DecrementInt (Variables|Default|GetAmmo2)
              (:%20%20
                (Math|Integer|DecrementInt (Variables|Default|GetAmmo)
                  (:%20%20
                    (Utilities|Array|SetArrayElem (Variables|/Game/Blueprints/Player/PlayerCharacterBP.PlayerCharacterBP_C|GetWeaponAmmo _as_player_character_bp_4) (Variables|/Game/Blueprints/Player/PlayerCharacterBP.PlayerCharacterBP_C|GetWeaponSlot _as_player_character_bp_4) (Variables|Default|GetAmmo))
                    (Utilities|FlowControl|Sequence
                      (:then_0
                        (bind _returnvalue_5 (Game|SpawnActorfromClass "/Game/Blueprints/FX/MuzzleFlash/StingerMuzzleFlashBP.StingerMuzzleFlashBP_C" (Transformation|GetWorldTransform _firepoint_2) "Undefined" "MultiplyWithRoot" 0 0))
                        (Transformation|AttachComponentToComponent _returnvalue_5 _firepoint_2 "None" "SnapToTarget" "SnapToTarget" "SnapToTarget" true)
                        (bind _outhit (Collision|LineTraceByChannel _returnvalue (+ _returnvalue (* (Math|Vector|GetForwardVector (Variables|/Game/Blueprints/Player/PlayerCharacterBP.PlayerCharacterBP_C|GetFollowCamera _as_player_character_bp_3)) (+ 8e+03 (Variables|/Game/Blueprints/Player/PlayerCharacterBP.PlayerCharacterBP_C|GetFireRange _as_player_character_bp_3)))) "TraceTypeQuery2" false 0 "None"))
                        (bind _asenemy_parent_bp (Utilities|Casting|CastToEnemyParentBP (.HitActor (Collision|BreakHitResult _outhit))))
                        (Default|TakeDamage _asenemy_parent_bp _returnvalue_3)
                        (bind _returnvalue_6 (UserInterface|CreateWidget "/Game/Widgets/Hud/DamageWidget.DamageWidget_C" 0 _returnvalue_3))
                        (UserInterface|Viewport|AddtoViewport _returnvalue_6 0))
                      (:then_1
                        (bind _returnvalue_7 (Game|SpawnActorfromClass "/Game/Blueprints/FX/MuzzleFlash/StingerMuzzleFlashBP.StingerMuzzleFlashBP_C" (Transformation|GetWorldTransform _firepoint2_2) "Undefined" "MultiplyWithRoot" 0 0))
                        (Transformation|AttachComponentToComponent _returnvalue_7 _firepoint2_2 "None" "SnapToTarget" "SnapToTarget" "SnapToTarget" true)
                        (bind _outhit_2 (Collision|LineTraceByChannel _returnvalue_2 (+ _returnvalue_2 (* (Math|Vector|GetForwardVector (Variables|/Game/Blueprints/Player/PlayerCharacterBP.PlayerCharacterBP_C|GetFollowCamera _as_player_character_bp_6)) (+ 8e+03 (Variables|/Game/Blueprints/Player/PlayerCharacterBP.PlayerCharacterBP_C|GetFireRange _as_player_character_bp_6)))) "TraceTypeQuery2" false 0 "None"))
                        (bind _asenemy_parent_bp_2 (Utilities|Casting|CastToEnemyParentBP (.HitActor (Collision|BreakHitResult _outhit_2))))
                        (Default|TakeDamage _asenemy_parent_bp_2 _returnvalue_4)
                        (bind _returnvalue_8 (UserInterface|CreateWidget "/Game/Widgets/Hud/DamageWidget.DamageWidget_C" 0 _returnvalue_4))
                        (UserInterface|Viewport|AddtoViewport _returnvalue_8 0))))))))
          (:OnNotifyBegin
            (Animation|Montage|PlayMontage _mesh "/Game/Models/Player/Animations/PlayerDualPistolHold_Montage.PlayerDualPistolHold_Montage"
              (:then
                (Variables|Default|SetFireCD false)))))
        (else
          (Utilities|FlowControl|DoOnce false :!label _label
            (:Completed
              (Variables|Default|SetReload? true)
              (Animation|Montage|PlayMontage _mesh_2 "/Game/Models/Player/Animations/PlayerReloadPistolBoth_Montage.PlayerReloadPistolBoth_Montage" (+ (Variables|/Game/Blueprints/Player/PlayerCharacterBP.PlayerCharacterBP_C|GetReloadSpeed (Variables|Default|GetAs%20Player%20Character%20BP)) 1.0)
                (:OnNotifyBegin
                  (Animation|Montage|PlayMontage _mesh_2 "/Game/Models/Player/Animations/PlayerDualPistolHold_Montage.PlayerDualPistolHold_Montage"
                    (:then
                      (bind _output_get (Variables|Default|SetAmmo (+ (Variables|/Game/Blueprints/Player/PlayerCharacterBP.PlayerCharacterBP_C|GetAmmo _as_player_character_bp_7) 20)))
                      (Variables|Default|SetAmmo2 (+ (Variables|/Game/Blueprints/Player/PlayerCharacterBP.PlayerCharacterBP_C|GetAmmo _as_player_character_bp_7) 20))
                      (Utilities|Array|SetArrayElem (Variables|/Game/Blueprints/Player/PlayerCharacterBP.PlayerCharacterBP_C|GetWeaponAmmo _as_player_character_bp_7) (Variables|/Game/Blueprints/Player/PlayerCharacterBP.PlayerCharacterBP_C|GetWeaponSlot _as_player_character_bp_7) _output_get)
                      (Utilities|FlowControl|Delay 0.2)
                      (Variables|Default|SetReload? false)
                      (Variables|Default|SetFireCD false)
                      (goto _label Reset)))))))))
      (else
        (goto _label)))))

(event EventScrollDown
  (bind _as_player_character_bp (Variables|Default|GetAs%20Player%20Character%20BP))
  (bind _as_player_character_bp_2 (Variables|Default|GetAs%20Player%20Character%20BP))
  (bind _firepoint (Variables|Default|GetFirePoint))
  (bind _as_player_character_bp_3 (Variables|Default|GetAs%20Player%20Character%20BP))
  (bind _firepoint2 (Variables|Default|GetFirePoint2))
  (bind _as_player_character_bp_4 (Variables|Default|GetAs%20Player%20Character%20BP))
  (bind _as_player_character_bp_5 (Variables|Default|GetAs%20Player%20Character%20BP))
  (bind _as_player_character_bp_6 (Variables|Default|GetAs%20Player%20Character%20BP))
  (bind _as_player_character_bp_7 (Variables|Default|GetAs%20Player%20Character%20BP))
  (bind _firepoint2_2 (Variables|Default|GetFirePoint2))
  (bind _as_player_character_bp_8 (Variables|Default|GetAs%20Player%20Character%20BP))
  (bind _firepoint_2 (Variables|Default|GetFirePoint))
  (bind _ocdamage (Variables|Default|GetOCDamage))
  (bind _ocdamage_2 (Variables|Default|GetOCDamage))
  (bind _returnvalue (Transformation|GetWorldLocation _firepoint))
  (bind _returnvalue_2 (Transformation|GetWorldLocation _firepoint2))
  (bind _damage (Variables|/Game/Blueprints/Player/PlayerCharacterBP.PlayerCharacterBP_C|GetDamage _as_player_character_bp_2))
  (bind _damage_2 (Variables|/Game/Blueprints/Player/PlayerCharacterBP.PlayerCharacterBP_C|GetDamage _as_player_character_bp_8))
  (bind _mesh (Variables|/Script/Engine.Character|GetMesh _as_player_character_bp_5))
  (bind _mesh_2 (Variables|/Script/Engine.Character|GetMesh _as_player_character_bp))
  (bind _returnvalue_3 (+ _damage_2 25 _ocdamage))
  (bind _returnvalue_4 (+ _damage 25 _ocdamage_2))
  (if (and (not (Variables|Default|GetFireCD)) (not (Variables|Default|GetReload?)))
    (if (> (Variables|Default|GetAmmo) 0)
      (if (> (Variables|Default|GetAmmo2) 0)
        (Animation|Montage|PlayMontage _mesh "/Game/Models/Player/Animations/PlayerDualPistolFireBoth_Montage.PlayerDualPistolFireBoth_Montage" (+ (Variables|/Game/Blueprints/Player/PlayerCharacterBP.PlayerCharacterBP_C|GetFireRate (Variables|Default|GetAs%20Player%20Character%20BP)) 1.65)
          (:then
            (Variables|Default|SetFireCD true)
            (Math|Integer|DecrementInt (Variables|Default|GetAmmo2)
              (:%20%20
                (Math|Integer|DecrementInt (Variables|Default|GetAmmo)
                  (:%20%20
                    (Utilities|Array|SetArrayElem (Variables|/Game/Blueprints/Player/PlayerCharacterBP.PlayerCharacterBP_C|GetWeaponAmmo _as_player_character_bp_4) (Variables|/Game/Blueprints/Player/PlayerCharacterBP.PlayerCharacterBP_C|GetWeaponSlot _as_player_character_bp_4) (Variables|Default|GetAmmo))
                    (Utilities|FlowControl|Sequence
                      (:then_0
                        (bind _returnvalue_5 (Game|SpawnActorfromClass "/Game/Blueprints/FX/MuzzleFlash/StingerMuzzleFlashBP.StingerMuzzleFlashBP_C" (Transformation|GetWorldTransform _firepoint_2) "Undefined" "MultiplyWithRoot" 0 0))
                        (Transformation|AttachComponentToComponent _returnvalue_5 _firepoint_2 "None" "SnapToTarget" "SnapToTarget" "SnapToTarget" true)
                        (bind _outhit (Collision|LineTraceByChannel _returnvalue (+ _returnvalue (* (Math|Vector|GetForwardVector (Variables|/Game/Blueprints/Player/PlayerCharacterBP.PlayerCharacterBP_C|GetFollowCamera _as_player_character_bp_3)) (+ 8e+03 (Variables|/Game/Blueprints/Player/PlayerCharacterBP.PlayerCharacterBP_C|GetFireRange _as_player_character_bp_3)))) "TraceTypeQuery2" false 0 "None"))
                        (bind _asenemy_parent_bp (Utilities|Casting|CastToEnemyParentBP (.HitActor (Collision|BreakHitResult _outhit))))
                        (Default|TakeDamage _asenemy_parent_bp _returnvalue_3)
                        (bind _returnvalue_6 (UserInterface|CreateWidget "/Game/Widgets/Hud/DamageWidget.DamageWidget_C" 0 _returnvalue_3))
                        (UserInterface|Viewport|AddtoViewport _returnvalue_6 0))
                      (:then_1
                        (bind _returnvalue_7 (Game|SpawnActorfromClass "/Game/Blueprints/FX/MuzzleFlash/StingerMuzzleFlashBP.StingerMuzzleFlashBP_C" (Transformation|GetWorldTransform _firepoint2_2) "Undefined" "MultiplyWithRoot" 0 0))
                        (Transformation|AttachComponentToComponent _returnvalue_7 _firepoint2_2 "None" "SnapToTarget" "SnapToTarget" "SnapToTarget" true)
                        (bind _outhit_2 (Collision|LineTraceByChannel _returnvalue_2 (+ _returnvalue_2 (* (Math|Vector|GetForwardVector (Variables|/Game/Blueprints/Player/PlayerCharacterBP.PlayerCharacterBP_C|GetFollowCamera _as_player_character_bp_6)) (+ 8e+03 (Variables|/Game/Blueprints/Player/PlayerCharacterBP.PlayerCharacterBP_C|GetFireRange _as_player_character_bp_6)))) "TraceTypeQuery2" false 0 "None"))
                        (bind _asenemy_parent_bp_2 (Utilities|Casting|CastToEnemyParentBP (.HitActor (Collision|BreakHitResult _outhit_2))))
                        (Default|TakeDamage _asenemy_parent_bp_2 _returnvalue_4)
                        (bind _returnvalue_8 (UserInterface|CreateWidget "/Game/Widgets/Hud/DamageWidget.DamageWidget_C" 0 _returnvalue_4))
                        (UserInterface|Viewport|AddtoViewport _returnvalue_8 0))))))))
          (:OnNotifyBegin
            (Animation|Montage|PlayMontage _mesh "/Game/Models/Player/Animations/PlayerDualPistolHold_Montage.PlayerDualPistolHold_Montage"
              (:then
                (Variables|Default|SetFireCD false)))))
        (else
          (Utilities|FlowControl|DoOnce false :!label _label
            (:Completed
              (Variables|Default|SetReload? true)
              (Animation|Montage|PlayMontage _mesh_2 "/Game/Models/Player/Animations/PlayerReloadPistolBoth_Montage.PlayerReloadPistolBoth_Montage" (+ (Variables|/Game/Blueprints/Player/PlayerCharacterBP.PlayerCharacterBP_C|GetReloadSpeed (Variables|Default|GetAs%20Player%20Character%20BP)) 1.0)
                (:OnNotifyBegin
                  (Animation|Montage|PlayMontage _mesh_2 "/Game/Models/Player/Animations/PlayerDualPistolHold_Montage.PlayerDualPistolHold_Montage"
                    (:then
                      (bind _output_get (Variables|Default|SetAmmo (+ (Variables|/Game/Blueprints/Player/PlayerCharacterBP.PlayerCharacterBP_C|GetAmmo _as_player_character_bp_7) 20)))
                      (Variables|Default|SetAmmo2 (+ (Variables|/Game/Blueprints/Player/PlayerCharacterBP.PlayerCharacterBP_C|GetAmmo _as_player_character_bp_7) 20))
                      (Utilities|Array|SetArrayElem (Variables|/Game/Blueprints/Player/PlayerCharacterBP.PlayerCharacterBP_C|GetWeaponAmmo _as_player_character_bp_7) (Variables|/Game/Blueprints/Player/PlayerCharacterBP.PlayerCharacterBP_C|GetWeaponSlot _as_player_character_bp_7) _output_get)
                      (Utilities|FlowControl|Delay 0.2)
                      (Variables|Default|SetReload? false)
                      (Variables|Default|SetFireCD false)
                      (goto _label Reset)))))))))
      (else
        (goto _label)))))

(event EventReload
  (bind _as_player_character_bp (Variables|Default|GetAs%20Player%20Character%20BP))
  (bind _as_player_character_bp_2 (Variables|Default|GetAs%20Player%20Character%20BP))
  (bind _as_player_character_bp_3 (Variables|Default|GetAs%20Player%20Character%20BP))
  (bind _mesh (Variables|/Script/Engine.Character|GetMesh _as_player_character_bp))
  (if (and (or (<= (Variables|Default|GetAmmo) (+ (Variables|/Game/Blueprints/Player/PlayerCharacterBP.PlayerCharacterBP_C|GetAmmo _as_player_character_bp_2) 19)) (<= (Variables|Default|GetAmmo2) (+ (Variables|/Game/Blueprints/Player/PlayerCharacterBP.PlayerCharacterBP_C|GetAmmo _as_player_character_bp_2) 19))) (not (Variables|/Game/Blueprints/Player/PlayerCharacterBP.PlayerCharacterBP_C|GetSwappingWeapons _as_player_character_bp_2)))
    (Utilities|FlowControl|DoOnce false :!label _label
      (:Completed
        (Variables|Default|SetReload? true)
        (Animation|Montage|PlayMontage _mesh "/Game/Models/Player/Animations/PlayerReloadPistolBoth_Montage.PlayerReloadPistolBoth_Montage" (+ (Variables|/Game/Blueprints/Player/PlayerCharacterBP.PlayerCharacterBP_C|GetReloadSpeed _as_player_character_bp_2) 1.0)
          (:OnNotifyBegin
            (Animation|Montage|PlayMontage _mesh "/Game/Models/Player/Animations/PlayerDualPistolHold_Montage.PlayerDualPistolHold_Montage"
              (:then
                (bind _output_get (Variables|Default|SetAmmo (+ (Variables|/Game/Blueprints/Player/PlayerCharacterBP.PlayerCharacterBP_C|GetAmmo _as_player_character_bp_3) 20)))
                (Variables|Default|SetAmmo2 (+ (Variables|/Game/Blueprints/Player/PlayerCharacterBP.PlayerCharacterBP_C|GetAmmo _as_player_character_bp_3) 20))
                (Utilities|Array|SetArrayElem (Variables|/Game/Blueprints/Player/PlayerCharacterBP.PlayerCharacterBP_C|GetWeaponAmmo _as_player_character_bp_3) (Variables|/Game/Blueprints/Player/PlayerCharacterBP.PlayerCharacterBP_C|GetWeaponSlot _as_player_character_bp_3) _output_get)
                (Utilities|FlowControl|Delay 0.2)
                (Variables|Default|SetReload? false)
                (Variables|Default|SetFireCD false)
                (goto _label Reset)))))))))

(fn ConstructionScript
  (|CallParentFunction))