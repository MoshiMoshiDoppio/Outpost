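; Player rocket launcher weapon that attaches to the character's WeaponSocket2, shows an ammo widget and fires rocket projectiles from its fire point.
; Montage notifies pace firing and reloading, with play rates and magazine size scaled by the player's stats.
; Ammo syncs to the player's weapon-slot array, and an empty magazine or Reload event runs a DoOnce-guarded reload.
; Right-click manually detonates the first rocket found in the world.
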(event EventBeginPlay
  (|CallParentFunction)
  (bind _asplayer_character_bp (Utilities|Casting|CastToPlayerCharacterBP (Game|GetPlayerCharacter 0)))
  (Variables|Default|SetAmmo (+ (Variables|/Game/Blueprints/Player/PlayerCharacterBP.PlayerCharacterBP_C|GetAmmo _asplayer_character_bp) 5))
  (Variables|Default|SetAs%20Player%20Character%20BP _asplayer_character_bp)
  (Animation|Montage|PlayMontage (Variables|/Script/Engine.Character|GetMesh _asplayer_character_bp) "/Game/Models/Player/Animations/PlayerHoldRocketLauncher_Montage.PlayerHoldRocketLauncher_Montage" 1.3
    (:then
      (Transformation|AttachComponentToComponent (Variables|/Script/Engine.Character|GetMesh _asplayer_character_bp) "WeaponSocket2" "SnapToTarget" "KeepRelative" "KeepWorld" true)
      (bind _returnvalue (UserInterface|CreateWidget "/Game/Widgets/Ammo/StingerAmmoWidget.StingerAmmoWidget_C"))
      (UserInterface|Viewport|AddtoViewport _returnvalue 0))))

(event EventRemoveWidget
  (Widget|RemovefromParent (stale EventBeginPlay _returnvalue)))

(event EventReload
  (bind _as_player_character_bp (Variables|Default|GetAs%20Player%20Character%20BP))
  (bind _as_player_character_bp_2 (Variables|Default|GetAs%20Player%20Character%20BP))
  (bind _as_player_character_bp_3 (Variables|Default|GetAs%20Player%20Character%20BP))
  (bind _mesh (Variables|/Script/Engine.Character|GetMesh _as_player_character_bp))
  (if (and (<= (Variables|Default|GetAmmo) (+ (Variables|/Game/Blueprints/Player/PlayerCharacterBP.PlayerCharacterBP_C|GetAmmo _as_player_character_bp_2) 4)) (not (Variables|/Game/Blueprints/Player/PlayerCharacterBP.PlayerCharacterBP_C|GetSwappingWeapons _as_player_character_bp_2)))
    (Utilities|FlowControl|DoOnce false :!label _label
      (:Completed
        (Variables|Default|SetReload? true)
        (Animation|Montage|PlayMontage _mesh "/Game/Models/Player/Animations/PlayerReloadRocketLauncher_Montage.PlayerReloadRocketLauncher_Montage" (+ (Variables|/Game/Blueprints/Player/PlayerCharacterBP.PlayerCharacterBP_C|GetReloadSpeed _as_player_character_bp_3) 1.0)
          (:OnNotifyBegin
            (Animation|Montage|PlayMontage _mesh "/Game/Models/Player/Animations/PlayerHoldRocketLauncher_Montage.PlayerHoldRocketLauncher_Montage" 1.3
              (:then
                (bind _output_get (Variables|Default|SetAmmo (+ (Variables|/Game/Blueprints/Player/PlayerCharacterBP.PlayerCharacterBP_C|GetAmmo _as_player_character_bp_3) 5)))
                (Utilities|Array|SetArrayElem (Variables|/Game/Blueprints/Player/PlayerCharacterBP.PlayerCharacterBP_C|GetWeaponAmmo _as_player_character_bp_3) (Variables|/Game/Blueprints/Player/PlayerCharacterBP.PlayerCharacterBP_C|GetWeaponSlot _as_player_character_bp_3) _output_get)
                (Utilities|FlowControl|Delay 0.2)
                (Variables|Default|SetReload? false)
                (Variables|Default|SetFireCD false)
                (goto _label Reset)))))))))

(event EventLeftClick
  (bind _as_player_character_bp (Variables|Default|GetAs%20Player%20Character%20BP))
  (bind _as_player_character_bp_2 (Variables|Default|GetAs%20Player%20Character%20BP))
  (bind _as_player_character_bp_3 (Variables|Default|GetAs%20Player%20Character%20BP))
  (bind _mesh (Variables|/Script/Engine.Character|GetMesh _as_player_character_bp))
  (if (> (Variables|Default|GetAmmo) 0)
    (if (Math|Boolean|ANDBoolean (not (Variables|Default|GetFireCD)) (not (Variables|Default|GetReload?)) (not (Variables|/Game/Blueprints/Player/PlayerCharacterBP.PlayerCharacterBP_C|GetSwappingWeapons (Variables|Default|GetAs%20Player%20Character%20BP))))
      (Variables|Default|SetFireCD true)
      (Animation|Montage|PlayMontage _mesh "/Game/Models/Player/Animations/PlayerFireRocketLauncher_Montage.PlayerFireRocketLauncher_Montage" (+ (Variables|/Game/Blueprints/Player/PlayerCharacterBP.PlayerCharacterBP_C|GetFireRate _as_player_character_bp) 1.0)
        (:then
          (bind _result (Math|Integer|DecrementInt (Variables|Default|GetAmmo))
            (:%20%20
              (Utilities|Array|SetArrayElem (Variables|/Game/Blueprints/Player/PlayerCharacterBP.PlayerCharacterBP_C|GetWeaponAmmo _as_player_character_bp_3) (Variables|/Game/Blueprints/Player/PlayerCharacterBP.PlayerCharacterBP_C|GetWeaponSlot _as_player_character_bp_3) _result)
              (Game|SpawnActorfromClass "/Game/Blueprints/Weapons/RocketProjectileBP.RocketProjectileBP_C" (Transformation|GetWorldTransform (Variables|Default|GetFirePoint)) "Undefined" "MultiplyWithRoot" 0 0))))
        (:OnNotifyBegin
          (if (== (Variables|Default|GetAmmo) 0)
            (Utilities|FlowControl|DoOnce false :!label _label
              (:Completed
                (Variables|Default|SetReload? true)
                (Animation|Montage|PlayMontage _mesh "/Game/Models/Player/Animations/PlayerReloadRocketLauncher_Montage.PlayerReloadRocketLauncher_Montage" (+ (Variables|/Game/Blueprints/Player/PlayerCharacterBP.PlayerCharacterBP_C|GetReloadSpeed _as_player_character_bp_2) 1.0)
                  (:OnNotifyBegin
                    (Animation|Montage|PlayMontage _mesh "/Game/Models/Player/Animations/PlayerHoldRocketLauncher_Montage.PlayerHoldRocketLauncher_Montage" 1.3
                      (:then
                        (bind _output_get (Variables|Default|SetAmmo (+ (Variables|/Game/Blueprints/Player/PlayerCharacterBP.PlayerCharacterBP_C|GetAmmo _as_player_character_bp_2) 5)))
                        (Utilities|Array|SetArrayElem (Variables|/Game/Blueprints/Player/PlayerCharacterBP.PlayerCharacterBP_C|GetWeaponAmmo _as_player_character_bp_2) (Variables|/Game/Blueprints/Player/PlayerCharacterBP.PlayerCharacterBP_C|GetWeaponSlot _as_player_character_bp_2) _output_get)
                        (Utilities|FlowControl|Delay 0.2)
                        (Variables|Default|SetReload? false)
                        (Variables|Default|SetFireCD false)
                        (goto _label Reset)))))))
            (else
              (Animation|Montage|PlayMontage _mesh "/Game/Models/Player/Animations/PlayerHoldRocketLauncher_Montage.PlayerHoldRocketLauncher_Montage" 1.3
                (:then
                  (Variables|Default|SetFireCD false))))))))
    (else
      (goto _label))))

(event EventRightClick
  (bind _outactors (Actor|GetAllActorsOfClass "/Game/Blueprints/Weapons/RocketProjectileBP.RocketProjectileBP_C"))
  (bind _array_element (Utilities|Array|ForEachLoopwithBreak _outactors :!label _label)
    (:LoopBody
      (Default|ManualExplode _array_element)
      (goto _label Break))))

(fn ConstructionScript
  (|CallParentFunction))