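; Player rocket projectile that explodes in a radius, damaging enemies and launching the player if caught in the blast.
; On spawn it ignores collision with the player, then after a short delay doubles its velocity and enables its light and trail.
; Hit and manual detonation share one path: spawn ExplosionBP, sphere-trace, then destroy itself.
; Each actor, deduplicated by name, takes player-based bonus damage with a damage widget, or receives velocity-boosted knockback.
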(event Custom|Explode
  (params (Location :type Vector))
  (bind _as_player_character_bp (Variables|Default|GetAs%20Player%20Character%20BP))
  (bind _hitactors (Variables|Default|GetHitActors))
  (bind _damage (Variables|/Game/Blueprints/Player/PlayerCharacterBP.PlayerCharacterBP_C|GetDamage _as_player_character_bp))
  (bind _returnvalue (+ _damage 500))
  (Variables|Default|SetHitLocation Location)
  (Game|SpawnActorfromClass "/Game/Materials/FX/ExplosionBP.ExplosionBP_C" (Transformation|GetActorTransform) "Undefined" "MultiplyWithRoot" 0 0)
  (bind _outhits (Collision|MultiSphereTraceByChannel (Variables|Default|GetHitLocation) (Variables|Default|GetHitLocation) 6e+02 "TraceTypeQuery2" false 0 "None"))
  (for _array_element _outhits
    (if (not (Utilities|Array|ContainsItem _hitactors (Utilities|GetDisplayName (.HitActor (Collision|BreakHitResult _array_element)))))
      (Utilities|Array|Add _hitactors (Utilities|GetDisplayName (.HitActor (Collision|BreakHitResult _array_element))))
      (Utilities|FlowControl|Sequence
        (:then_0
          (bind _asenemy_parent_bp (Utilities|Casting|CastToEnemyParentBP (.HitActor (Collision|BreakHitResult _array_element))))
          (Default|TakeDamage _asenemy_parent_bp _returnvalue)
          (bind _returnvalue_2 (UserInterface|CreateWidget "/Game/Widgets/Hud/DamageWidget.DamageWidget_C" 0 _returnvalue))
          (UserInterface|Viewport|AddtoViewport _returnvalue_2 0))
        (:then_1
          (bind _asplayer_character_bp (Utilities|Casting|CastToPlayerCharacterBP (.HitActor (Collision|BreakHitResult _array_element))))
          (Default|SetVelocity _asplayer_character_bp (* (.x (Transformation|GetVelocity _asplayer_character_bp)) 2.0) (* (.y (Transformation|GetVelocity _asplayer_character_bp)) 2.0) (Math|Float|Clamp(Float) (.z (Transformation|GetVelocity _asplayer_character_bp)) 0.0 1e+05))
          (Character|LaunchCharacter _asplayer_character_bp (Math|Vector|MakeVector (.x (* (Math|Vector|Normalize (- (Variables|Default|GetHitLocation) (Transformation|GetActorLocation))) -3e+03)) (.y (* (Math|Vector|Normalize (- (Variables|Default|GetHitLocation) (Transformation|GetActorLocation))) -3e+03)) (* (.z (* (Math|Vector|Normalize (- (Variables|Default|GetHitLocation) (Transformation|GetActorLocation))) -3e+03)) 1.35)) false false)))))
  (Actor|DestroyActor))

(event Custom|ManualExplode
  (bind _as_player_character_bp (Variables|Default|GetAs%20Player%20Character%20BP))
  (bind _hitactors (Variables|Default|GetHitActors))
  (bind _damage (Variables|/Game/Blueprints/Player/PlayerCharacterBP.PlayerCharacterBP_C|GetDamage _as_player_character_bp))
  (bind _returnvalue (+ _damage 500))
  (Variables|Default|SetHitLocation (Transformation|GetActorLocation))
  (Game|SpawnActorfromClass "/Game/Materials/FX/ExplosionBP.ExplosionBP_C" (Transformation|GetActorTransform) "Undefined" "MultiplyWithRoot" 0 0)
  (bind _outhits (Collision|MultiSphereTraceByChannel (Variables|Default|GetHitLocation) (Variables|Default|GetHitLocation) 6e+02 "TraceTypeQuery2" false 0 "None"))
  (for _array_element _outhits
    (if (not (Utilities|Array|ContainsItem _hitactors (Utilities|GetDisplayName (.HitActor (Collision|BreakHitResult _array_element)))))
      (Utilities|Array|Add _hitactors (Utilities|GetDisplayName (.HitActor (Collision|BreakHitResult _array_element))))
      (Utilities|FlowControl|Sequence
        (:then_0
          (bind _asenemy_parent_bp (Utilities|Casting|CastToEnemyParentBP (.HitActor (Collision|BreakHitResult _array_element))))
          (Default|TakeDamage _asenemy_parent_bp _returnvalue)
          (bind _returnvalue_2 (UserInterface|CreateWidget "/Game/Widgets/Hud/DamageWidget.DamageWidget_C" 0 _returnvalue))
          (UserInterface|Viewport|AddtoViewport _returnvalue_2 0))
        (:then_1
          (bind _asplayer_character_bp (Utilities|Casting|CastToPlayerCharacterBP (.HitActor (Collision|BreakHitResult _array_element))))
          (Default|SetVelocity _asplayer_character_bp (* (.x (Transformation|GetVelocity _asplayer_character_bp)) 2.0) (* (.y (Transformation|GetVelocity _asplayer_character_bp)) 2.0) (Math|Float|Clamp(Float) (.z (Transformation|GetVelocity _asplayer_character_bp)) 0.0 1e+05))
          (Character|LaunchCharacter _asplayer_character_bp (Math|Vector|MakeVector (.x (* (Math|Vector|Normalize (- (Variables|Default|GetHitLocation) (Transformation|GetActorLocation))) -3e+03)) (.y (* (Math|Vector|Normalize (- (Variables|Default|GetHitLocation) (Transformation|GetActorLocation))) -3e+03)) (* (.z (* (Math|Vector|Normalize (- (Variables|Default|GetHitLocation) (Transformation|GetActorLocation))) -3e+03)) 1.35)) false false)))))
  (Actor|DestroyActor))

(event EventBeginPlay
  (bind _projectilemovement (Variables|Default|GetProjectileMovement))
  (bind _asplayer_character_bp (Utilities|Casting|CastToPlayerCharacterBP (Game|GetPlayerCharacter 0)))
  (Variables|Default|SetAs%20Player%20Character%20BP _asplayer_character_bp)
  (Collision|IgnoreActorwhenMoving (Variables|Default|GetCollision) _asplayer_character_bp true)
  (Collision|IgnoreActorwhenMoving (Variables|/Script/Engine.Character|GetCapsuleComponent _asplayer_character_bp) self true)
  (Utilities|FlowControl|Delay 0.3)
  (Variables|/Script/Engine.MovementComponent|SetVelocity _projectilemovement (* (Variables|/Script/Engine.MovementComponent|GetVelocity _projectilemovement) 2.0))
  (Rendering|SetVisibility (Variables|Default|GetPointLight) true false)
  (Effects|SpawnEmitterAttached "/Game/FX/RocketTrail/RocketTrailFX.RocketTrailFX" (Variables|Default|GetRocketTrail) "None"))

(event Collision|EventHit
  (params (MyComp :type Primitive%20Component%20Object%20Reference) (Other :type Actor%20Object%20Reference) (OtherComp :type Primitive%20Component%20Object%20Reference) (bSelfMoved :type Boolean) (HitLocation :type Vector :default "0, 0, 0") (HitNormal :type Vector :default "0, 0, 0") (NormalImpulse :type Vector :default "0, 0, 0") (Hit :type Hit%20Result%20Structure%20%28by%20ref%29))
  (CallFunction|Explode HitLocation))

(fn ConstructionScript)