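; Player laser sword weapon that attaches to the character's WeaponSocket and swaps to a white laser material when that upgrade is owned.
; Left and right click play different attack montages at a speed based on the player's FireRate, each setting its own DamageX value.
; A cooldown flag and weapon-swap check gate attacks; the montage's notify restores the hold pose and clears the cooldown.
; Hit detection is not handled in this graph.
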(event EventBeginPlay
  (|CallParentFunction)
  (Variables|Default|SetAmmo 1)
  (bind _asoagame_instance (Utilities|Casting|CastToOAGameInstance (Game|GetGameInstance)))
  (if (Utilities|Array|ContainsItem (Variables|/Game/Blueprints/GamemodeInstance/OAGameInstance.OAGameInstance_C|GetPlayerWeaponUpgrades _asoagame_instance) "WhiteLaser")
    (Rendering|Material|SetMaterial (Variables|Default|GetStaticMesh) 1 "/Game/Materials/WhiteLaserMat.WhiteLaserMat"))
  (bind _asplayer_character_bp (Utilities|Casting|CastToPlayerCharacterBP (Game|GetPlayerCharacter 0)))
  (Variables|Default|SetAs%20Player%20Character%20BP _asplayer_character_bp)
  (Animation|Montage|PlayMontage (Variables|/Script/Engine.Character|GetMesh _asplayer_character_bp) "/Game/Models/Player/Animations/PlayerHoldSword_Montage.PlayerHoldSword_Montage"
    (:then
      (Transformation|AttachComponentToComponent (Variables|/Script/Engine.Character|GetMesh _asplayer_character_bp) "WeaponSocket" "SnapToTarget" "KeepRelative" "KeepWorld" true))))

(event Collision|EventActorBeginOverlap
  (params (OtherActor :type Actor%20Object%20Reference))
  (|CallParentFunction OtherActor) ; This node is disabled and will not be called.\nDrag off pins to build functionality.
)

(event EventTick
  (params (DeltaSeconds :type Float%20%28single-precision%29))
  (|CallParentFunction DeltaSeconds) ; This node is disabled and will not be called.\nDrag off pins to build functionality.
)

(event EventLeftClick
  (bind _as_player_character_bp (Variables|Default|GetAs%20Player%20Character%20BP))
  (bind _mesh (Variables|/Script/Engine.Character|GetMesh _as_player_character_bp))
  (if (and (not (Variables|Default|GetFireCD)) (not (Variables|/Game/Blueprints/Player/PlayerCharacterBP.PlayerCharacterBP_C|GetSwappingWeapons (Variables|Default|GetAs%20Player%20Character%20BP))))
    (Variables|Default|SetFireCD true)
    (Animation|Montage|PlayMontage _mesh "/Game/Models/Player/Animations/PlayerSwordAttack1_Montage.PlayerSwordAttack1_Montage" (+ (Variables|/Game/Blueprints/Player/PlayerCharacterBP.PlayerCharacterBP_C|GetFireRate _as_player_character_bp) 1.0)
      (:then
        (Variables|Default|SetDamageX 2.0))
      (:OnNotifyBegin
        (Animation|Montage|PlayMontage _mesh "/Game/Models/Player/Animations/PlayerHoldSword_Montage.PlayerHoldSword_Montage"
          (:then
            (Variables|Default|SetFireCD false)))))))

(event EventRightClick
  (bind _as_player_character_bp (Variables|Default|GetAs%20Player%20Character%20BP))
  (bind _mesh (Variables|/Script/Engine.Character|GetMesh _as_player_character_bp))
  (if (and (not (Variables|Default|GetFireCD)) (not (Variables|/Game/Blueprints/Player/PlayerCharacterBP.PlayerCharacterBP_C|GetSwappingWeapons (Variables|Default|GetAs%20Player%20Character%20BP))))
    (Variables|Default|SetFireCD true)
    (Animation|Montage|PlayMontage _mesh "/Game/Models/Player/Animations/PlayerSwordAttack2_Montage.PlayerSwordAttack2_Montage" (+ (Variables|/Game/Blueprints/Player/PlayerCharacterBP.PlayerCharacterBP_C|GetFireRate _as_player_character_bp) 1.0)
      (:then
        (Variables|Default|SetDamageX 1.5))
      (:OnNotifyBegin
        (Animation|Montage|PlayMontage _mesh "/Game/Models/Player/Animations/PlayerHoldSword_Montage.PlayerHoldSword_Montage"
          (:then
            (Variables|Default|SetFireCD false)))))))

(fn ConstructionScript
  (|CallParentFunction))