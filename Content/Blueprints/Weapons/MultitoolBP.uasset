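; Multitool weapon that attaches to the player's hand socket and lets them identify and name aliens, reusing pistol montages.
; A looping 0.1-second timer traces from the fire point toward the camera's aim, using a DoOnce to show the targeted alien's name widget until the aim leaves it.
; Left click repeats the trace to open a naming widget on the hit alien, with a cooldown cleared by the fire montage's notify.
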(event Custom|Trace
  (bind _as_player_character_bp (Variables|Default|GetAs%20Player%20Character%20BP))
  (bind _followcamera (Variables|/Game/Blueprints/Player/PlayerCharacterBP.PlayerCharacterBP_C|GetFollowCamera _as_player_character_bp))
  (Utilities|Time|SetTimerbyEvent (delegate Custom|Trace) 0.1 true)
  (bind (_outhit _returnvalue) (Collision|LineTraceByChannel (Transformation|GetWorldLocation (Variables|Default|GetFirePoint)) (+ (Transformation|GetWorldLocation _followcamera) (* (Math|Vector|GetForwardVector _followcamera) 4e+03)) "TraceTypeQuery2" false 0 "None"))
  (if _returnvalue
    (bind _asenemy_parent_bp (Utilities|Casting|CastToEnemyParentBP (.HitActor (Collision|BreakHitResult _outhit)))
      (:then
        (Utilities|FlowControl|DoOnce false :!label _label
          (:Completed
            (bind _returnvalue_2 (UserInterface|CreateWidget "/Game/Widgets/Ammo/MultitoolWidget.MultitoolWidget_C" 0 (Variables|/Game/Blueprints/Enemies/EnemyParentBP.EnemyParentBP_C|GetName _asenemy_parent_bp)))
            (UserInterface|Viewport|AddtoViewport _returnvalue_2 0))))
      (:CastFailed
        (Utilities|IsValid _returnvalue_2 :!label _label_2
          (:Is%20Valid
            (Widget|RemovefromParent _returnvalue_2)
            (goto _label Reset)))))
    (else
      (goto _label_2))))

(event EventBeginPlay
  (|CallParentFunction)
  (Variables|Default|SetAmmo 1)
  (bind _asplayer_character_bp (Utilities|Casting|CastToPlayerCharacterBP (Game|GetPlayerCharacter 0)))
  (Variables|Default|SetAs%20Player%20Character%20BP _asplayer_character_bp)
  (Animation|Montage|PlayMontage (Variables|/Script/Engine.Character|GetMesh _asplayer_character_bp) "/Game/Models/Player/Animations/PlayerHoldPistol_Montage.PlayerHoldPistol_Montage"
    (:then
      (Transformation|AttachComponentToComponent (Variables|/Script/Engine.Character|GetMesh _asplayer_character_bp) "WeaponSocket" "SnapToTarget" "KeepRelative" "KeepWorld" true)
      (CallFunction|Trace))))

(event Collision|EventActorBeginOverlap
  (params (OtherActor :type Actor%20Object%20Reference))
  (|CallParentFunction OtherActor) ; This node is disabled and will not be called.\nDrag off pins to build functionality.
)

(event EventTick
  (params (DeltaSeconds :type Float%20%28single-precision%29))
  (|CallParentFunction DeltaSeconds) ; This node is disabled and will not be called.\nDrag off pins to build functionality.
)

(event EventLeftClick
  (bind _as_player_character_bp (Variables|Default|GetAs%20Player%20Character%20BP))
  (bind _as_player_character_bp_2 (Variables|Default|GetAs%20Player%20Character%20BP))
  (bind _mesh (Variables|/Script/Engine.Character|GetMesh _as_player_character_bp))
  (bind _followcamera (Variables|/Game/Blueprints/Player/PlayerCharacterBP.PlayerCharacterBP_C|GetFollowCamera _as_player_character_bp_2))
  (if (Math|Boolean|ANDBoolean (not (Variables|Default|GetFireCD)) (not (Variables|Default|GetReload?)) (not (Variables|/Game/Blueprints/Player/PlayerCharacterBP.PlayerCharacterBP_C|GetSwappingWeapons (Variables|Default|GetAs%20Player%20Character%20BP))))
    (Variables|Default|SetFireCD true)
    (Animation|Montage|PlayMontage _mesh "/Game/Models/Player/Animations/PlayerPistolFire_Montage.PlayerPistolFire_Montage" 1.2
      (:then
        (bind (_outhit _returnvalue) (Collision|LineTraceByChannel (Transformation|GetWorldLocation (Variables|Default|GetFirePoint)) (+ (Transformation|GetWorldLocation _followcamera) (* (Math|Vector|GetForwardVector _followcamera) 4e+03)) "TraceTypeQuery2" false 0 "None"))
        (if _returnvalue
          (bind _asenemy_parent_bp (Utilities|Casting|CastToEnemyParentBP (.HitActor (Collision|BreakHitResult _outhit))))
          (bind _returnvalue_2 (UserInterface|CreateWidget "/Game/Widgets/Ammo/AlienNamingWidget.AlienNamingWidget_C" 0 (Variables|/Game/Blueprints/Enemies/EnemyParentBP.EnemyParentBP_C|GetName _asenemy_parent_bp) (.HitActor (Collision|BreakHitResult _outhit))))
          (UserInterface|Viewport|AddtoViewport _returnvalue_2 0)
          (Utilities|IsValid (stale Custom|Trace _returnvalue_2)
            (:Is%20Valid
              (Widget|RemovefromParent (stale Custom|Trace _returnvalue_2))
              (Utilities|FlowControl|DoOnce false) ; enters at Reset
            ))))
      (:OnNotifyBegin
        (Animation|Montage|PlayMontage _mesh "/Game/Models/Player/Animations/PlayerHoldPistol_Montage.PlayerHoldPistol_Montage"
          (:then
            (Variables|Default|SetFireCD false)))))))

(fn ConstructionScript
  (|CallParentFunction))