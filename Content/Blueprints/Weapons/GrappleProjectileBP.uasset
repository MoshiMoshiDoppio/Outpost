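; Grapple gun projectile that pulls the player toward its hit point.
; On spawn it applies the faster-firing upgrade, ignores player collision and starts timers that grow Distance until Hit and trigger the gun's LeftClick beyond cable length.
; Launch toggles pulling through a debounced FlipFlop.
; Pull re-arms a looping timer that repeatedly launches the character along hit direction plus camera forward, destroying the projectile on weapon swap.
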(event Custom|CheckDistance
  (bind _returnvalue (Utilities|Time|SetTimerbyEvent (delegate Custom|CheckDistance) 0.1 true))
  (Variables|Default|SetDistance (Math|Float|Clamp(Float) (+ (Variables|Default|GetDistance) 0.2) 1.0 5.0)))

(event Custom|Launch
  (Utilities|FlowControl|Sequence
    (:then_0
      (Utilities|FlowControl|DoOnce false :!label _label
        (:Completed
          (Utilities|FlowControl|FlipFlop
            (:A
              (CallFunction|Pull))
            (:B
              (CallFunction|StopPull))))))
    (:then_1
      (Utilities|FlowControl|Delay 0.3)
      (goto _label Reset))))

(event Custom|Pull
  (bind _hit_location (Variables|Default|GetHit%20Location))
  (bind _as_player_character_bp (Variables|Default|GetAs%20Player%20Character%20BP))
  (bind _as_grapple_gun_bp (Variables|Default|GetAs%20Grapple%20Gun%20BP))
  (bind _returnvalue (Transformation|GetActorLocation _as_player_character_bp))
  (bind _grappleforce (Variables|/Game/Blueprints/Weapons/GrappleGunBP.GrappleGunBP_C|GetGrappleForce _as_grapple_gun_bp))
  (bind _followcamera (Variables|/Game/Blueprints/Player/PlayerCharacterBP.PlayerCharacterBP_C|GetFollowCamera _as_player_character_bp))
  (bind _returnvalue_2 (Math|Rotator|FindLookatRotation _returnvalue _hit_location))
  (bind _returnvalue_3 (Math|Vector|GetForwardVector _followcamera))
  (bind _returnvalue_4 (Math|Rotator|GetRotationXVector _returnvalue_2))
  (bind _returnvalue_5 (* _returnvalue_3 2e+02))
  (bind _returnvalue_6 (* _returnvalue_4 4.5e+02))
  (bind _returnvalue_7 (* _returnvalue_6 _grappleforce))
  (bind _returnvalue_8 (Utilities|Time|SetTimerbyEvent (delegate Custom|Pull) 0.05 true))
  (if (Variables|/Game/Blueprints/Player/PlayerCharacterBP.PlayerCharacterBP_C|GetSwappingWeapons (Variables|Default|GetAs%20Player%20Character%20BP))
    (CallFunction|StopPull)
    (Actor|DestroyActor)
    (else
      (Character|LaunchCharacter _as_player_character_bp (Math|Vector|MakeVector (+ (.x _returnvalue_5) (.x _returnvalue_7)) (+ (.y _returnvalue_5) (.y _returnvalue_7)) (* (.z _returnvalue_7) 1.2)) false false))))

(event Custom|StopPull
  (Utilities|Time|ClearandInvalidateTimerbyHandle (stale Custom|Pull _returnvalue_8)))

(event Custom|CheckCableLength
  (bind _as_grapple_gun_bp (Variables|Default|GetAs%20Grapple%20Gun%20BP))
  (bind _returnvalue (Utilities|Time|SetTimerbyEvent (delegate Custom|CheckCableLength) 0.1 true))
  (if (> (Math|Vector|VectorLength (- (Transformation|GetActorLocation (Variables|Default|GetAs%20Player%20Character%20BP)) (Transformation|GetActorLocation))) (Variables|/Game/Blueprints/Weapons/GrappleGunBP.GrappleGunBP_C|GetCableLength _as_grapple_gun_bp))
    (Utilities|Time|ClearandInvalidateTimerbyHandle _returnvalue)
    (Default|LeftClick _as_grapple_gun_bp)))

(event EventBeginPlay
  (bind _projectilemovement (Variables|Default|GetProjectileMovement))
  (bind _asoagame_instance (Utilities|Casting|CastToOAGameInstance (Game|GetGameInstance)))
  (if (Utilities|Array|ContainsItem (Variables|/Game/Blueprints/GamemodeInstance/OAGameInstance.OAGameInstance_C|GetPlayerWeaponUpgrades _asoagame_instance) "FasterFiring")
    (Variables|/Script/Engine.MovementComponent|SetVelocity _projectilemovement (* (Variables|/Script/Engine.MovementComponent|GetVelocity _projectilemovement) 2.5)))
  (bind _asplayer_character_bp (Utilities|Casting|CastToPlayerCharacterBP (Game|GetPlayerCharacter 0)))
  (Variables|Default|SetAs%20Player%20Character%20BP _asplayer_character_bp)
  (bind _asgrapple_gun_bp (Utilities|Casting|CastToGrappleGunBP (Variables|/Game/Blueprints/Player/PlayerCharacterBP.PlayerCharacterBP_C|GetWeapon _asplayer_character_bp)))
  (Variables|Default|SetAs%20Grapple%20Gun%20BP _asgrapple_gun_bp)
  (Collision|IgnoreActorwhenMoving (Variables|Default|GetCollision) _asplayer_character_bp true)
  (Collision|IgnoreActorwhenMoving (Variables|/Script/Engine.Character|GetCapsuleComponent _asplayer_character_bp) self true)
  (CallFunction|CheckDistance)
  (CallFunction|CheckCableLength))

(event Collision|EventHit
  (params (MyComp :type Primitive%20Component%20Object%20Reference) (Other :type Actor%20Object%20Reference) (OtherComp :type Primitive%20Component%20Object%20Reference) (bSelfMoved :type Boolean) (HitLocation :type Vector :default "0, 0, 0") (HitNormal :type Vector :default "0, 0, 0") (NormalImpulse :type Vector :default "0, 0, 0") (Hit :type Hit%20Result%20Structure%20%28by%20ref%29))
  (Variables|Default|SetHit%20Location HitLocation)
  (Utilities|Time|ClearandInvalidateTimerbyHandle (stale Custom|CheckDistance _returnvalue))
  (Variables|Default|SetHit true))

(fn ConstructionScript)