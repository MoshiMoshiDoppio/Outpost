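; Player grapple gun weapon that fires a cabled projectile along the camera's forward vector and triggers its launch once it hits.
; Left click alternates firing and destroying projectiles, debounced by a 0.4-second DoOnce reset; right click calls Launch on hit projectiles.
; Scroll adjusts a clamped GrappleForce.
; BeginPlay applies the LongerCable upgrade from the game instance, attaches the gun to the character's weapon socket and creates a strength widget.
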(event EventBeginPlay
  (|CallParentFunction)
  (bind _asoagame_instance (Utilities|Casting|CastToOAGameInstance (Game|GetGameInstance)))
  (if (Utilities|Array|ContainsItem (Variables|/Game/Blueprints/GamemodeInstance/OAGameInstance.OAGameInstance_C|GetPlayerWeaponUpgrades _asoagame_instance) "LongerCable")
    (Variables|Default|SetCableLength 2.05e+04))
  (bind _asplayer_character_bp (Utilities|Casting|CastToPlayerCharacterBP (Game|GetPlayerCharacter 0)))
  (Variables|Default|SetAs%20Player%20Character%20BP _asplayer_character_bp)
  (Animation|Montage|PlayMontage (Variables|/Script/Engine.Character|GetMesh _asplayer_character_bp) "/Game/Models/Player/Animations/PlayerHoldGrapple_Montage.PlayerHoldGrapple_Montage"
    (:then
      (Transformation|AttachComponentToComponent (Variables|/Script/Engine.Character|GetMesh _asplayer_character_bp) "WeaponSocket" "SnapToTarget" "KeepRelative" "KeepWorld" true)
      (bind _returnvalue (UserInterface|CreateWidget "/Game/Widgets/Ammo/GrappleStrengthWidget.GrappleStrengthWidget_C"))
      (UserInterface|Viewport|AddtoViewport _returnvalue 0))))

(event EventRightClick
  (if (Variables|Default|GetFireCD)
    (bind _outactors (Actor|GetAllActorsOfClass "/Game/Blueprints/Weapons/GrappleProjectileBP.GrappleProjectileBP_C"))
    (for _array_element _outactors
      (if (Variables|/Game/Blueprints/Weapons/GrappleProjectileBP.GrappleProjectileBP_C|GetHit _array_element)
        (Default|Launch _array_element)))))

(event EventScrollUp
  (Variables|Default|SetGrappleForce (Math|Float|Clamp(Float) (+ (Variables|Default|GetGrappleForce) 0.1) 0.31 1.5)))

(event EventLeftClick
  (bind _as_player_character_bp (Variables|Default|GetAs%20Player%20Character%20BP))
  (bind _staticmesh1 (Variables|Default|GetStaticMesh1))
  (bind _cable (Variables|Default|GetCable))
  (bind _firepoint (Variables|Default|GetFirePoint))
  (bind _returnvalue (Transformation|GetWorldTransform _firepoint))
  (bind _mesh (Variables|/Script/Engine.Character|GetMesh _as_player_character_bp))
  (Utilities|FlowControl|Sequence
    (:then_0
      (Utilities|FlowControl|DoOnce false :!label _label
        (:Completed
          (Utilities|FlowControl|FlipFlop
            (:A
              (if (and (not (Variables|Default|GetFireCD)) (not (Variables|/Game/Blueprints/Player/PlayerCharacterBP.PlayerCharacterBP_C|GetSwappingWeapons (Variables|Default|GetAs%20Player%20Character%20BP))))
                (Rendering|SetVisibility _staticmesh1 false false)
                (Variables|Default|SetFireCD true)
                (Animation|Montage|PlayMontage _mesh "/Game/Models/Player/Animations/PlayerFireGrapple_Montage.PlayerFireGrapple_Montage"
                  (:then
                    (bind _returnvalue_2 (Game|SpawnActorfromClass "/Game/Blueprints/Weapons/GrappleProjectileBP.GrappleProjectileBP_C" (Math|Transform|MakeTransform (.location _returnvalue) (Math|Conversions|RotationFromXVector (Math|Vector|GetForwardVector (Variables|/Game/Blueprints/Player/PlayerCharacterBP.PlayerCharacterBP_C|GetFollowCamera (Variables|Default|GetAs%20Player%20Character%20BP)))) (.scale _returnvalue)) "Undefined" "MultiplyWithRoot" 0 0))
                    (Variables|Default|SetGrappleProjectile _returnvalue_2)
                    (Class|CableComponent|SetAttachEndtoComponent _cable (Variables|/Game/Blueprints/Weapons/GrappleProjectileBP.GrappleProjectileBP_C|GetCablePoint _returnvalue_2) "None")
                    (Rendering|SetVisibility _cable true false))
                  (:OnNotifyBegin
                    (Animation|Montage|PlayMontage _mesh "/Game/Models/Player/Animations/PlayerHoldGrapple_Montage.PlayerHoldGrapple_Montage")))))
            (:B
              (bind _outactors (Actor|GetAllActorsOfClass "/Game/Blueprints/Weapons/GrappleProjectileBP.GrappleProjectileBP_C"))
              (for _array_element _outactors
                (Actor|DestroyActor _array_element)
                (Rendering|SetVisibility (Variables|Default|GetCable) false false)
                (Variables|Default|SetFireCD false)
                (Rendering|SetVisibility _staticmesh1 true false)))))))
    (:then_1
      (Utilities|FlowControl|Delay 0.4)
      (goto _label Reset))))

(event EventScrollDown
  (Variables|Default|SetGrappleForce (Math|Float|Clamp(Float) (- (Variables|Default|GetGrappleForce) 0.1) 0.31 1.5)))

(event EventRemoveWidget
  (Utilities|IsValid (stale EventBeginPlay _returnvalue)
    (:Is%20Valid
      (Widget|RemovefromParent (stale EventBeginPlay _returnvalue)))))

(fn ConstructionScript
  (|CallParentFunction))