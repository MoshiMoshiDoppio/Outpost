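; Pincher hitscan gun that attaches to the player's weapon socket and shows an ammo widget.
; Left click traces from the fire point along the camera's forward vector, damages enemies with a damage widget, and spawns a muzzle flash.
; Player stats modify magazine size, fire rate, range, damage and reload speed.
; Montage notifies clear the fire cooldown and drive automatic or manual reloads through a shared DoOnce, syncing ammo to the player's slot array.
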(event EventBeginPlay
  (|CallParentFunction)
  (Variables|Default|SetFireRate 1.0)
  (bind _asplayer_character_bp (Utilities|Casting|CastToPlayerCharacterBP (Game|GetPlayerCharacter 0)))
  (Variables|Default|SetAmmo (+ (Variables|/Game/Blueprints/Player/PlayerCharacterBP.PlayerCharacterBP_C|GetAmmo _asplayer_character_bp) 45))
  (Variables|Default|SetAs%20Player%20Character%20BP _asplayer_character_bp)
  (Animation|Montage|PlayMontage (Variables|/Script/Engine.Character|GetMesh _asplayer_character_bp) "/Game/Models/Player/Animations/PlayerHoldPincher_Montage.PlayerHoldPincher_Montage"
    (:then
      (Transformation|AttachComponentToComponent (Variables|/Script/Engine.Character|GetMesh _asplayer_character_bp) "WeaponSocket" "SnapToTarget" "KeepRelative" "KeepWorld" true)
      (bind _returnvalue (UserInterface|CreateWidget "/Game/Widgets/Ammo/StingerAmmoWidget.StingerAmmoWidget_C"))
      (UserInterface|Viewport|AddtoViewport _returnvalue 0))))

(event EventRemoveWidget
  (Utilities|IsValid (stale EventBeginPlay _returnvalue)
    (:Is%20Valid
      (Widget|RemovefromParent (stale EventBeginPlay _returnvalue)))))

(event EventReload
  (bind _as_player_character_bp (Variables|Default|GetAs%20Player%20Character%20BP))
  (bind _as_player_character_bp_2 (Variables|Default|GetAs%20Player%20Character%20BP))
  (bind _as_player_character_bp_3 (Variables|Default|GetAs%20Player%20Character%20BP))
  (bind _mesh (Variables|/Script/Engine.Character|GetMesh _as_player_character_bp))
  (if (and (<= (Variables|Default|GetAmmo) (+ (Variables|/Game/Blueprints/Player/PlayerCharacterBP.PlayerCharacterBP_C|GetAmmo _as_player_character_bp_2) 44)) (not (Variables|/Game/Blueprints/Player/PlayerCharacterBP.PlayerCharacterBP_C|GetSwappingWeapons _as_player_character_bp_2)))
    (Utilities|FlowControl|DoOnce false :!label _label
      (:Completed
        (Variables|Default|SetReload? true)
        (Animation|Montage|PlayMontage _mesh "/Game/Models/Player/Animations/PlayerReloadPistolLeft_Montage.PlayerReloadPistolLeft_Montage" (+ (Variables|/Game/Blueprints/Player/PlayerCharacterBP.PlayerCharacterBP_C|GetReloadSpeed _as_player_character_bp_3) 1.0)
          (:OnNotifyBegin
            (Animation|Montage|PlayMontage _mesh "/Game/Models/Player/Animations/PlayerHoldPincher_Montage.PlayerHoldPincher_Montage"
              (:then
                (bind _output_get (Variables|Default|SetAmmo (+ (Variables|/Game/Blueprints/Player/PlayerCharacterBP.PlayerCharacterBP_C|GetAmmo _as_player_character_bp_3) 45)))
                (Utilities|Array|SetArrayElem (Variables|/Game/Blueprints/Player/PlayerCharacterBP.PlayerCharacterBP_C|GetWeaponAmmo _as_player_character_bp_3) (Variables|/Game/Blueprints/Player/PlayerCharacterBP.PlayerCharacterBP_C|GetWeaponSlot _as_player_character_bp_3) _output_get)
                (Utilities|FlowControl|Delay 0.2)
                (Variables|Default|SetReload? false)
                (Variables|Default|SetFireCD false)
                (goto _label Reset)))))))))

(event EventLeftClick
  (bind _as_player_character_bp (Variables|Default|GetAs%20Player%20Character%20BP))
  (bind _as_player_character_bp_2 (Variables|Default|GetAs%20Player%20Character%20BP))
  (bind _as_player_character_bp_3 (Variables|Default|GetAs%20Player%20Character%20BP))
  (bind _as_player_character_bp_4 (Variables|Default|GetAs%20Player%20Character%20BP))
  (bind _firepoint (Variables|Default|GetFirePoint))
  (bind _as_player_character_bp_5 (Variables|Default|GetAs%20Player%20Character%20BP))
  (bind _firepoint_2 (Variables|Default|GetFirePoint))
  (bind _returnvalue (Transformation|GetWorldLocation _firepoint))
  (bind _damage (Variables|/Game/Blueprints/Player/PlayerCharacterBP.PlayerCharacterBP_C|GetDamage _as_player_character_bp_2))
  (bind _mesh (Variables|/Script/Engine.Character|GetMesh _as_player_character_bp))
  (bind _returnvalue_2 (+ _damage 100))
  (if (> (Variables|Default|GetAmmo) 0)
    (if (Math|Boolean|ANDBoolean (not (Variables|Default|GetFireCD)) (not (Variables|Default|GetReload?)) (not (Variables|/Game/Blueprints/Player/PlayerCharacterBP.PlayerCharacterBP_C|GetSwappingWeapons (Variables|Default|GetAs%20Player%20Character%20BP))))
      (Variables|Default|SetFireCD true)
      (Animation|Montage|PlayMontage _mesh "/Game/Models/Player/Animations/PlayerFirePincher_Montage.PlayerFirePincher_Montage" (Math|Float|Clamp(Float) (+ (Variables|/Game/Blueprints/Player/PlayerCharacterBP.PlayerCharacterBP_C|GetFireRate _as_player_character_bp) (Variables|Default|GetFireRate)) 0.0 1.7)
        (:then
          (bind _result (Math|Integer|DecrementInt (Variables|Default|GetAmmo))
            (:%20%20
              (Utilities|Array|SetArrayElem (Variables|/Game/Blueprints/Player/PlayerCharacterBP.PlayerCharacterBP_C|GetWeaponAmmo _as_player_character_bp_4) (Variables|/Game/Blueprints/Player/PlayerCharacterBP.PlayerCharacterBP_C|GetWeaponSlot _as_player_character_bp_4) _result)
              (bind _returnvalue_3 (Game|SpawnActorfromClass "/Game/Blueprints/FX/MuzzleFlash/StingerMuzzleFlashBP.StingerMuzzleFlashBP_C" (Transformation|GetWorldTransform _firepoint_2) "Undefined" "MultiplyWithRoot" 0 0))
              (Transformation|AttachComponentToComponent _returnvalue_3 _firepoint_2 "None" "SnapToTarget" "SnapToTarget" "SnapToTarget" true)
              (bind _outhit (Collision|LineTraceByChannel _returnvalue (+ _returnvalue (* (Math|Vector|GetForwardVector (Variables|/Game/Blueprints/Player/PlayerCharacterBP.PlayerCharacterBP_C|GetFollowCamera _as_player_character_bp_5)) (+ 1.2e+04 (Variables|/Game/Blueprints/Player/PlayerCharacterBP.PlayerCharacterBP_C|GetFireRange _as_player_character_bp_5)))) "TraceTypeQuery2" false 0 "None"))
              (bind _asenemy_parent_bp (Utilities|Casting|CastToEnemyParentBP (.HitActor (Collision|BreakHitResult _outhit))))
              (Default|TakeDamage _asenemy_parent_bp _returnvalue_2)
              (bind _returnvalue_4 (UserInterface|CreateWidget "/Game/Widgets/Hud/DamageWidget.DamageWidget_C" 0 _returnvalue_2))
              (UserInterface|Viewport|AddtoViewport _returnvalue_4 0))))
        (:OnNotifyBegin
          (if (== _result 0)
            (Utilities|FlowControl|DoOnce false :!label _label
              (:Completed
                (Variables|Default|SetReload? true)
                (Animation|Montage|PlayMontage _mesh "/Game/Models/Player/Animations/PlayerReloadPistolLeft_Montage.PlayerReloadPistolLeft_Montage" (+ (Variables|/Game/Blueprints/Player/PlayerCharacterBP.PlayerCharacterBP_C|GetReloadSpeed _as_player_character_bp_3) 1.0)
                  (:OnNotifyBegin
                    (Animation|Montage|PlayMontage _mesh "/Game/Models/Player/Animations/PlayerHoldPincher_Montage.PlayerHoldPincher_Montage"
                      (:then
                        (bind _output_get (Variables|Default|SetAmmo (+ (Variables|/Game/Blueprints/Player/PlayerCharacterBP.PlayerCharacterBP_C|GetAmmo _as_player_character_bp_3) 45)))
                        (Utilities|Array|SetArrayElem (Variables|/Game/Blueprints/Player/PlayerCharacterBP.PlayerCharacterBP_C|GetWeaponAmmo _as_player_character_bp_3) (Variables|/Game/Blueprints/Player/PlayerCharacterBP.PlayerCharacterBP_C|GetWeaponSlot _as_player_character_bp_3) _output_get)
                        (Utilities|FlowControl|Delay 0.2)
                        (Variables|Default|SetReload? false)
                        (Variables|Default|SetFireCD false)
                        (goto _label Reset)))))))
            (else
              (Animation|Montage|PlayMontage _mesh "/Game/Models/Player/Animations/PlayerHoldPincher_Montage.PlayerHoldPincher_Montage"
                (:then
                  (Variables|Default|SetFireCD false))))))))
    (else
      (goto _label))))

(fn ConstructionScript
  (|CallParentFunction))