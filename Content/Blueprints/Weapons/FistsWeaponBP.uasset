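; Fists weapon Blueprint that plays melee animations on the player character, cached at BeginPlay.
; Left and right clicks play their respective punch montages, while scrolling either way plays an OraOra montage if the player's OraOra flag is set.
; A shared FireCD flag blocks new attacks until a montage notify clears it and plays the idle montage.
; Playback speed scales with the player's FireRate, within clamped limits.
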(event EventBeginPlay
  (|CallParentFunction)
  (Variables|Default|SetFireRate 1.0)
  (bind _asplayer_character_bp (Utilities|Casting|CastToPlayerCharacterBP (Game|GetPlayerCharacter 0)))
  (bind _output_get (Variables|Default|SetAs%20Player%20Character%20BP _asplayer_character_bp))
  (Animation|StopAnimMontage (Variables|Default|GetAs%20Player%20Character%20BP) 0))

(event Collision|EventActorBeginOverlap
  (params (OtherActor :type Actor%20Object%20Reference))
  (|CallParentFunction OtherActor) ; This node is disabled and will not be called.\nDrag off pins to build functionality.
)

(event EventLeftClick
  (bind _as_player_character_bp (Variables|Default|GetAs%20Player%20Character%20BP))
  (bind _mesh (Variables|/Script/Engine.Character|GetMesh _as_player_character_bp))
  (if (not (Variables|Default|GetFireCD))
    (Animation|Montage|PlayMontage _mesh "/Game/Models/Player/Animations/PlayerLeftPunch_Montage.PlayerLeftPunch_Montage" (Math|Float|Clamp(Float) (+ (Variables|/Game/Blueprints/Player/PlayerCharacterBP.PlayerCharacterBP_C|GetFireRate _as_player_character_bp) 1.0) 1.0 1.8)
      (:then
        (Variables|Default|SetFireCD true))
      (:OnNotifyBegin
        (Variables|Default|SetFireCD false)
        (Animation|Montage|PlayMontage _mesh "/Game/Models/Player/Animations/PlayerIdle_Montage.PlayerIdle_Montage")))))

(event EventRightClick
  (bind _as_player_character_bp (Variables|Default|GetAs%20Player%20Character%20BP))
  (bind _mesh (Variables|/Script/Engine.Character|GetMesh _as_player_character_bp))
  (if (not (Variables|Default|GetFireCD))
    (Animation|Montage|PlayMontage _mesh "/Game/Models/Player/Animations/PlayerRightPunch_Montage.PlayerRightPunch_Montage" (Math|Float|Clamp(Float) (+ (Variables|/Game/Blueprints/Player/PlayerCharacterBP.PlayerCharacterBP_C|GetFireRate _as_player_character_bp) 1.0) 1.0 1.8)
      (:then
        (Variables|Default|SetFireCD true))
      (:OnNotifyBegin
        (Variables|Default|SetFireCD false)
        (Animation|Montage|PlayMontage _mesh "/Game/Models/Player/Animations/PlayerIdle_Montage.PlayerIdle_Montage")))))

(event EventScrollUp
  (bind _as_player_character_bp (Variables|Default|GetAs%20Player%20Character%20BP))
  (bind _mesh (Variables|/Script/Engine.Character|GetMesh _as_player_character_bp))
  (if (not (Variables|Default|GetFireCD))
    (if (Variables|/Game/Blueprints/Player/PlayerCharacterBP.PlayerCharacterBP_C|GetOraOra (Variables|Default|GetAs%20Player%20Character%20BP))
      (Animation|Montage|PlayMontage _mesh "/Game/Models/Player/Animations/PlayerOraOra_Montage.PlayerOraOra_Montage" (Math|Float|Clamp(Float) (+ (Variables|/Game/Blueprints/Player/PlayerCharacterBP.PlayerCharacterBP_C|GetFireRate (Variables|Default|GetAs%20Player%20Character%20BP)) (Variables|Default|GetFireRate)) 0.0 1.8)
        (:then
          (Variables|Default|SetFireCD true))
        (:OnNotifyBegin
          (Variables|Default|SetFireCD false)
          (Animation|Montage|PlayMontage _mesh "/Game/Models/Player/Animations/PlayerIdle_Montage.PlayerIdle_Montage"))))))

(event EventScrollDown
  (bind _as_player_character_bp (Variables|Default|GetAs%20Player%20Character%20BP))
  (bind _mesh (Variables|/Script/Engine.Character|GetMesh _as_player_character_bp))
  (if (not (Variables|Default|GetFireCD))
    (if (Variables|/Game/Blueprints/Player/PlayerCharacterBP.PlayerCharacterBP_C|GetOraOra (Variables|Default|GetAs%20Player%20Character%20BP))
      (Animation|Montage|PlayMontage _mesh "/Game/Models/Player/Animations/PlayerOraOra_Montage.PlayerOraOra_Montage" (Math|Float|Clamp(Float) (+ (Variables|/Game/Blueprints/Player/PlayerCharacterBP.PlayerCharacterBP_C|GetFireRate (Variables|Default|GetAs%20Player%20Character%20BP)) (Variables|Default|GetFireRate)) 0.0 1.8)
        (:then
          (Variables|Default|SetFireCD true))
        (:OnNotifyBegin
          (Variables|Default|SetFireCD false)
          (Animation|Montage|PlayMontage _mesh "/Game/Models/Player/Animations/PlayerIdle_Montage.PlayerIdle_Montage"))))))

(fn ConstructionScript
  (|CallParentFunction))