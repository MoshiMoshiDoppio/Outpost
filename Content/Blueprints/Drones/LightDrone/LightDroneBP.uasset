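; Light drone Blueprint that keeps its altitude tracking about 100 units above the player character.
; On BeginPlay it caches the player as PlayerCharacterBP and calls CheckHeight, which re-arms its own fast looping timer on each run.
; Each tick of that timer steps the drone up or down by a fixed amount toward the target height, with no dead zone and no change to X or Y.
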(event Custom|CheckHeight
  (bind _returnvalue (Transformation|GetActorLocation))
  (Utilities|Time|SetTimerbyEvent (delegate Custom|CheckHeight) 0.01 true)
  (bind _output_get (Variables|Default|SetDesiredHeight (+ (.z (Transformation|GetActorLocation (Variables|Default|GetAs%20Player%20Character%20BP))) 1e+02)))
  (if (> _output_get (.z _returnvalue))
    (Transformation|SetActorLocation (Math|Vector|MakeVector (.x _returnvalue) (.y _returnvalue) (+ (.z _returnvalue) 2.0)) false false)
    (else
      (Transformation|SetActorLocation (Math|Vector|MakeVector (.x _returnvalue) (.y _returnvalue) (- (.z _returnvalue) 2.0)) false false))))

(event EventBeginPlay
  (bind _asplayer_character_bp (Utilities|Casting|CastToPlayerCharacterBP (Game|GetPlayerCharacter 0)))
  (Variables|Default|SetAs%20Player%20Character%20BP _asplayer_character_bp)
  (CallFunction|CheckHeight))

(fn ConstructionScript
  (|CallParentFunction))