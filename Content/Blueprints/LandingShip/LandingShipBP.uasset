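; Landing ship interactable that lets the player sleep unless a hostile enemy is chasing.
; A 0.1-second looping timer scans all EnemyParentBP actors, stopping at the first hostile chaser to set BeingChased and switch Name between "Sleep" and "Being Pursued".
; Interact creates SleepWidget and adds it to the viewport only while BeingChased is false.
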(event Custom|Interact
  (if (not (Variables|Default|GetBeingChased))
    (bind _returnvalue (UserInterface|CreateWidget "/Game/Widgets/Sleep/SleepWidget.SleepWidget_C"))
    (UserInterface|Viewport|AddtoViewport _returnvalue 0)))

(event Custom|CheckIfChased
  (Utilities|Time|SetTimerbyEvent (delegate Custom|CheckIfChased) 0.1 true)
  (bind _outactors (Actor|GetAllActorsOfClass "/Game/Blueprints/Enemies/EnemyParentBP.EnemyParentBP_C"))
  (bind _array_element (Utilities|Array|ForEachLoopwithBreak _outactors :!label _label)
    (:LoopBody
      (if (Variables|/Game/Blueprints/Enemies/EnemyParentBP.EnemyParentBP_C|GetHostile _array_element)
        (if (Variables|/Game/Blueprints/Enemies/EnemyParentBP.EnemyParentBP_C|GetChasing _array_element)
          (Variables|Default|SetName "Being Pursued")
          (Variables|Default|SetBeingChased true)
          (goto _label Break)
          (else
            _)))
      (Variables|Default|SetName "Sleep")
      (Variables|Default|SetBeingChased false))))

(event EventBeginPlay
  (Variables|Default|SetName "Sleep")
  (CallFunction|CheckifChased))

(fn ConstructionScript)