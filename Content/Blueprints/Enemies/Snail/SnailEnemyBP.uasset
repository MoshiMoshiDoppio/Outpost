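; Snail enemy that players damage for credits, with a name shared across all snails via the game instance.
; A looping timer shrinks its PawnSensing sight radius by the player's Stealth, and further while crouched.
; Damage triggers Alert and Chase on nearby snails, driving an exclamation icon and a timed SeenPlayer blackboard flag.
; Non-lethal hits pay credits out of its bounty, and death pays the remainder.
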(event Custom|Alert
  (bind _exclamation (Variables|Default|GetExclamation))
  (Utilities|FlowControl|DoOnce false
    (:Completed
      (Rendering|SetVisibility _exclamation true false)
      (Utilities|FlowControl|Delay 0.6)
      (Rendering|SetVisibility _exclamation false false))))

(event Custom|Chase
  (bind _returnvalue (Utilities|Name|MakeLiteralName "SeenPlayer"))
  (bind _self self)
  (bind _exclamation (Variables|Default|GetExclamation))
  (bind _returnvalue_2 (AI|GetAIController _self))
  (bind _returnvalue_3 (AI|GetBlackboard _returnvalue_2))
  (Utilities|FlowControl|Sequence
    (:then_0
      (AI|Components|Blackboard|SetValueasBool _returnvalue_3 _returnvalue true))
    (:then_1
      (Utilities|FlowControl|RetriggerableDelay 1e+01)
      (AI|Components|Blackboard|SetValueasBool _returnvalue_3 _returnvalue false)
      (Utilities|FlowControl|DoOnce false) ; enters at Reset
    )))

(event Custom|CheckPlayerCrouch
  (bind _pawnsensing (Variables|Default|GetPawnSensing))
  (Utilities|Time|SetTimerbyEvent (delegate Custom|CheckPlayerCrouch) 0.1 true)
  (bind _asplayer_character_bp (Utilities|Casting|CastToPlayerCharacterBP (Game|GetPlayerCharacter 0)))
  (if (Variables|/Script/Engine.Character|GetbIsCrouched _asplayer_character_bp)
    (Utilities|FlowControl|DoOnce false :!label _label
      (:Completed
        (Variables|/Script/AIModule.PawnSensingComponent|SetSightRadius _pawnsensing (Math|Float|Clamp(Float) (- 3e+03 (Variables|/Game/Blueprints/Player/PlayerCharacterBP.PlayerCharacterBP_C|GetStealth _asplayer_character_bp)) 0.0 999999.0))
        (goto _label_2 Reset)))
    (else
      (Utilities|FlowControl|DoOnce false :!label _label_2
        (:Completed
          (Variables|/Script/AIModule.PawnSensingComponent|SetSightRadius _pawnsensing (Math|Float|Clamp(Float) (- 5e+03 (Variables|/Game/Blueprints/Player/PlayerCharacterBP.PlayerCharacterBP_C|GetStealth _asplayer_character_bp)) 0.0 999999.0))
          (goto _label Reset))))))

(event EventBeginPlay
  (bind _asoagame_instance (Utilities|Casting|CastToOAGameInstance (Game|GetGameInstance)))
  (Variables|Default|SetAs%20OAGame%20Instance _asoagame_instance)
  (Variables|Default|SetName (Variables|/Game/Blueprints/GamemodeInstance/OAGameInstance.OAGameInstance_C|GetSnailName _asoagame_instance))
  (Variables|Default|SetHealth 200)
  (Variables|Default|SetValue 150)
  (CallFunction|CheckPlayerCrouch))

(event EventTakeDamage
  (params (DMG :type Integer))
  (bind _output_get (Variables|Default|SetHealth (- (Variables|Default|GetHealth) DMG)))
  (bind _outactors (Actor|GetAllActorsOfClass "SnailEnemyBP_C"))
  (for _array_element _outactors
    (if (<= (Transformation|GetDistanceTo _array_element self) 5e+03)
      (CallFunction|Alert _array_element)
      (CallFunction|Chase _array_element)))
  (if (<= _output_get 0)
    (bind _asoagame_instance (Utilities|Casting|CastToOAGameInstance (Game|GetGameInstance)))
    (Variables|/Game/Blueprints/GamemodeInstance/OAGameInstance.OAGameInstance_C|SetCredits _asoagame_instance (+ (Variables|/Game/Blueprints/GamemodeInstance/OAGameInstance.OAGameInstance_C|GetCredits _asoagame_instance) (Variables|Default|GetValue)))
    (Actor|DestroyActor)
    (else
      (CallFunction|Chase)
      (bind _asoagame_instance_2 (Utilities|Casting|CastToOAGameInstance (Game|GetGameInstance)))
      (Variables|/Game/Blueprints/GamemodeInstance/OAGameInstance.OAGameInstance_C|SetCredits _asoagame_instance_2 (+ (Variables|/Game/Blueprints/GamemodeInstance/OAGameInstance.OAGameInstance_C|GetCredits _asoagame_instance_2) 35))
      (Variables|Default|SetValue (Math|Integer|Clamp(Integer) (- (Variables|Default|GetValue) 35) 0 999999)))))

(event EventSetName
  (bind _as_oagame_instance (Variables|Default|GetAs%20OAGame%20Instance))
  (Variables|/Game/Blueprints/GamemodeInstance/OAGameInstance.OAGameInstance_C|SetSnailName _as_oagame_instance (Variables|Default|GetName))
  (bind _outactors (Actor|GetAllActorsOfClass "SnailEnemyBP_C"))
  (for _array_element _outactors
    (Variables|/Game/Blueprints/Enemies/EnemyParentBP.EnemyParentBP_C|SetName _array_element (Variables|/Game/Blueprints/GamemodeInstance/OAGameInstance.OAGameInstance_C|GetSnailName _as_oagame_instance))))

(fn ConstructionScript
  (|CallParentFunction))