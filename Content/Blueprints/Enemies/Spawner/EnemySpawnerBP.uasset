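; EnemySpawnerBP is an enemy spawner actor that repeatedly spawns enemies at its own transform.
; After BeginPlay it waits a short random delay, then calls the Spawn event.
; Spawn re-arms its own looping timer with a random interval between LowerSpawn and UpperSpawn, so the spacing varies each cycle.
; Each call spawns only the first class in the Enemies array.
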(event Custom|Spawn
  (Utilities|Time|SetTimerbyEvent (delegate Custom|Spawn) (Math|Random|RandomFloatinRange (Variables|Default|GetLowerSpawn) (Variables|Default|GetUpperSpawn)) true)
  (Game|SpawnActorfromClass (Utilities|Array|Get(acopy) (Variables|Default|GetEnemies)) (Transformation|GetActorTransform) "Undefined" "MultiplyWithRoot" 0 0))

(event EventBeginPlay
  (Utilities|FlowControl|Delay (Math|Random|RandomFloatinRange 0.0 5.0))
  (CallFunction|Spawn))

(fn ConstructionScript)