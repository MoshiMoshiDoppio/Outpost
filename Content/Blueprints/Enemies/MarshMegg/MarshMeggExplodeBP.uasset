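; Explosion actor for the MarshMegg enemy that slows the player if caught in its blast.
; On BeginPlay it attaches the explosion particle effect and runs a single zero-length multi-sphere trace on the Camera channel around itself.
; The first PlayerCharacterBP among the hits gets its Slowed flag set and SetSlowed called.
; The actor destroys itself after a short delay, whether or not it finds a player.
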(event EventBeginPlay
  (bind _returnvalue (Transformation|GetActorLocation))
  (Effects|SpawnEmitterAttached "/Game/FX/MuzzleFlash/MarshMeggExplodeFX.MarshMeggExplodeFX" (Variables|Default|GetDefaultSceneRoot) "None")
  (bind (_outhits _returnvalue_2) (Collision|MultiSphereTraceByChannel _returnvalue _returnvalue 6e+02 "TraceTypeQuery2" false 0 "None"))
  (if _returnvalue_2
    (bind _array_element (Utilities|Array|ForEachLoopwithBreak _outhits :!label _label)
      (:LoopBody
        (bind _asplayer_character_bp (Utilities|Casting|CastToPlayerCharacterBP (.HitActor (Collision|BreakHitResult _array_element)))
          (:then
            (Variables|/Game/Blueprints/Player/PlayerCharacterBP.PlayerCharacterBP_C|SetSlowed _asplayer_character_bp true)
            (Default|SetSlowed _asplayer_character_bp)
            (goto _label Break))
          (:CastFailed
            _)))
      (:Completed
        _)))
  (Utilities|FlowControl|Delay 3.0)
  (Actor|DestroyActor))

(fn ConstructionScript)