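; Projectile fired by the Cyclops enemy that explodes on hit and deals heavy area damage to players.
; On spawn it and its Cyclops instigator ignore each other's movement collision.
; On hit it spawns a scaled explosion, sphere-traces around the impact, damages each player once by tracking actor names, then destroys itself.
; Knockback launch logic is present but disconnected.
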(event Custom|Explode
  (params (Location :type Vector))
  (bind _returnvalue (Transformation|GetActorTransform))
  (bind _hitactors (Variables|Default|GetHitActors))
  (Variables|Default|SetHitLocation Location)
  (Game|SpawnActorfromClass "/Game/Materials/FX/ExplosionBP.ExplosionBP_C" (Math|Transform|MakeTransform (.location _returnvalue) (.rotation _returnvalue) "1.100000,1.100000,1.100000") "Undefined" "MultiplyWithRoot" 0 0)
  (bind _outhits (Collision|MultiSphereTraceByChannel (Variables|Default|GetHitLocation) (Variables|Default|GetHitLocation) 1.1e+03 "TraceTypeQuery2" false 0 "None"))
  (for _array_element _outhits
    (if (not (Utilities|Array|ContainsItem _hitactors (Utilities|GetDisplayName (.HitActor (Collision|BreakHitResult _array_element)))))
      (Utilities|Array|Add _hitactors (Utilities|GetDisplayName (.HitActor (Collision|BreakHitResult _array_element))))
      (bind _asplayer_character_bp (Utilities|Casting|CastToPlayerCharacterBP (.HitActor (Collision|BreakHitResult _array_element))))
      (Default|TakeDamage _asplayer_character_bp 1000)
      (if (> (Variables|/Game/Blueprints/Player/PlayerCharacterBP.PlayerCharacterBP_C|GetHealth _asplayer_character_bp) 0)
        _)))
  (Actor|DestroyActor))

(event EventBeginPlay
  (bind _ascyclops_enemy_bp (Utilities|Casting|CastToCyclopsEnemyBP (Variables|Actor|GetInstigator)))
  (Collision|IgnoreActorwhenMoving (Variables|Default|GetCollision) _ascyclops_enemy_bp true)
  (Collision|IgnoreActorwhenMoving (Variables|/Script/Engine.Character|GetCapsuleComponent _ascyclops_enemy_bp) self true))

(event Collision|EventHit
  (params (MyComp :type Primitive%20Component%20Object%20Reference) (Other :type Actor%20Object%20Reference) (OtherComp :type Primitive%20Component%20Object%20Reference) (bSelfMoved :type Boolean) (HitLocation :type Vector :default "0, 0, 0") (HitNormal :type Vector :default "0, 0, 0") (NormalImpulse :type Vector :default "0, 0, 0") (Hit :type Hit%20Result%20Structure%20%28by%20ref%29))
  (CallFunction|Explode HitLocation))

(fn ConstructionScript)