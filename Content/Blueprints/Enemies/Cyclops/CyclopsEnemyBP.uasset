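; Hostile Cyclops enemy with a blinking lit eye that slams players in its hit box and fires projectiles while chasing.
; Pawn sensing, with sight radius adjusted for player crouch and Stealth, or damage triggers an alert to every Cyclops, as the distance check compares self to self.
; Chase sets the SeenPlayer blackboard key, with a retriggerable timeout that hits refresh.
; Hits pay credits from its bounty, and death pays the remainder.
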(event OnComponentBeginOverlap(HitBox)
  (params (OverlappedComponent :type Primitive%20Component%20Object%20Reference) (OtherActor :type Actor%20Object%20Reference) (OtherComp :type Primitive%20Component%20Object%20Reference) (OtherBodyIndex :type Integer) (bFromSweep :type Boolean) (SweepResult :type Hit%20Result%20Structure%20%28by%20ref%29))
  (Utilities|Casting|CastToPlayerCharacterBP OtherActor)
  (CallFunction|Attack)
  (CallFunction|Chase))

(event OnComponentEndOverlap(HitBox)
  (params (OverlappedComponent :type Primitive%20Component%20Object%20Reference) (OtherActor :type Actor%20Object%20Reference) (OtherComp :type Primitive%20Component%20Object%20Reference) (OtherBodyIndex :type Integer))
  (Utilities|Casting|CastToPlayerCharacterBP OtherActor)
  (Utilities|Time|ClearandInvalidateTimerbyHandle (stale Custom|Attack _returnvalue)))

(event OnSeePawn(PawnSensing)
  (params (Pawn :type Pawn%20Object%20Reference))
  (Utilities|Casting|CastToPlayerCharacterBP Pawn)
  (CallFunction|Alert))

(event Custom|Attack
  (bind _mesh (Variables|Character|GetMesh))
  (bind _charactermovement (Variables|Character|GetCharacterMovement))
  (bind _returnvalue (Utilities|Time|SetTimerbyEvent (delegate Custom|Attack) 5.0 true))
  (if (not (Variables|Default|GetAA))
    (Variables|Default|SetAA true)
    (Variables|/Script/Engine.CharacterMovementComponent|SetMaxWalkSpeed _charactermovement 0.0)
    (if (== (Math|Random|RandomIntegerinRange 0 1) 0)
      (Animation|Montage|PlayMontage _mesh "/Game/Models/Enemies/Cyclops/Animations/CyclopsSlam_Montage.CyclopsSlam_Montage"
        (:OnCompleted
          _))
      (else
        (Animation|Montage|PlayMontage _mesh "/Game/Models/Enemies/Cyclops/Animations/CyclopsSlam2_Montage.CyclopsSlam2_Montage"
          (:OnCompleted
            _))))
    (Variables|Default|SetAA false)
    (Variables|/Script/Engine.CharacterMovementComponent|SetMaxWalkSpeed _charactermovement 8e+02)))

(event Custom|Chase
  (bind _returnvalue (Utilities|Name|MakeLiteralName "SeenPlayer"))
  (bind _self self)
  (bind _exclamation (Variables|Default|GetExclamation))
  (bind _returnvalue_2 (AI|GetAIController _self))
  (bind _returnvalue_3 (AI|GetBlackboard _returnvalue_2))
  (Utilities|FlowControl|DoOnce false :!label _label
    (:Completed
      (Utilities|FlowControl|Sequence
        (:then_0
          (AI|Components|Blackboard|SetValueasBool _returnvalue_3 _returnvalue true)
          (Variables|Default|SetChasing true)
          (CallFunction|Attack2))
        (:then_1
          (Utilities|FlowControl|RetriggerableDelay 45.0)
          (AI|Components|Blackboard|SetValueasBool _returnvalue_3 _returnvalue false)
          (Variables|Default|SetChasing false)
          (Utilities|Time|ClearandInvalidateTimerbyHandle (stale Custom|Attack2 _returnvalue))
          (goto _label Reset))
        (:then_2
          (Rendering|SetVisibility _exclamation true false)
          (Utilities|FlowControl|Delay 0.6)
          (Rendering|SetVisibility _exclamation false false))))))

(event Custom|Attack2
  (bind _firepoint (Variables|Default|GetFirePoint))
  (bind _charactermovement (Variables|Character|GetCharacterMovement))
  (bind _returnvalue (Utilities|Time|SetTimerbyEvent (delegate Custom|Attack2) (Math|Random|RandomFloatinRange 5.0 1e+01) true))
  (if (not (Variables|Default|GetAA))
    (bind _asplayer_character_bp (Utilities|Casting|CastToPlayerCharacterBP (Game|GetPlayerCharacter 0)))
    (if (> (Math|Vector|DotProduct (Math|Vector|GetUnitDirection(Vector) (Transformation|GetActorLocation) (Transformation|GetActorLocation _asplayer_character_bp)) (Transformation|GetActorForwardVector)) 0.0)
      (Variables|Default|SetAA true)
      (Variables|/Script/Engine.CharacterMovementComponent|SetMaxWalkSpeed _charactermovement 0.0)
      (Animation|Montage|PlayMontage (Variables|Character|GetMesh) "/Game/Models/Enemies/Cyclops/Animations/CyclopsFire_Montage.CyclopsFire_Montage"
        (:OnCompleted
          (Variables|/Script/Engine.CharacterMovementComponent|SetMaxWalkSpeed _charactermovement 8e+02)
          (Variables|Default|SetAA false))
        (:OnNotifyBegin
          (Game|SpawnActorfromClass "/Game/Blueprints/Enemies/Cyclops/CyclopsProjectileBP.CyclopsProjectileBP_C" (Math|Transform|MakeTransform (.location (Transformation|GetWorldTransform _firepoint)) (Math|Rotator|FindLookatRotation (Transformation|GetWorldLocation _firepoint) (+ (Transformation|GetActorLocation (Game|GetPlayerCharacter 0)) (Math|Random|RandomFloatinRange -5.0 5.0))) "1.000000,1.000000,1.000000") "Undefined" "MultiplyWithRoot" 0 self))))))

(event Custom|CheckPlayerCrouch
  (bind _pawnsensing (Variables|Default|GetPawnSensing))
  (Utilities|Time|SetTimerbyEvent (delegate Custom|CheckPlayerCrouch) 0.1 true)
  (bind _asplayer_character_bp (Utilities|Casting|CastToPlayerCharacterBP (Game|GetPlayerCharacter 0)))
  (if (Variables|/Script/Engine.Character|GetbIsCrouched _asplayer_character_bp)
    (Utilities|FlowControl|DoOnce false :!label _label
      (:Completed
        (Variables|/Script/AIModule.PawnSensingComponent|SetSightRadius _pawnsensing (Math|Float|Clamp(Float) (- 3e+03 (Variables|/Game/Blueprints/Player/PlayerCharacterBP.PlayerCharacterBP_C|GetStealth _asplayer_character_bp)) 0.0 999999.0))
        (goto _label_2 Reset)))
    (else
      (Utilities|FlowControl|DoOnce false :!label _label_2
        (:Completed
          (Variables|/Script/AIModule.PawnSensingComponent|SetSightRadius _pawnsensing (Math|Float|Clamp(Float) (- 5e+03 (Variables|/Game/Blueprints/Player/PlayerCharacterBP.PlayerCharacterBP_C|GetStealth _asplayer_character_bp)) 0.0 999999.0))
          (goto _label Reset))))))

(event Custom|Alert
  (bind _outactors (Actor|GetAllActorsOfClass "CyclopsEnemyBP_C"))
  (for _array_element _outactors
    (if (<= (Transformation|GetDistanceTo self) 5e+03)
      (CallFunction|Chase _array_element))))

(event Custom|Blink
  (bind _sphere (Variables|Default|GetSphere))
  (Utilities|Time|SetTimerbyEvent (delegate Custom|Blink) (Math|Random|RandomFloatinRange 4.0 8.0) true)
  (Rendering|SetVisibility _sphere false false)
  (Utilities|FlowControl|Delay 1.0)
  (Rendering|SetVisibility _sphere true false))

(event EventBeginPlay
  (Variables|Default|SetHostile true)
  (bind _asoagame_instance (Utilities|Casting|CastToOAGameInstance (Game|GetGameInstance)))
  (Variables|Default|SetAs%20OAGame%20Instance _asoagame_instance)
  (Variables|Default|SetName (Variables|/Game/Blueprints/GamemodeInstance/OAGameInstance.OAGameInstance_C|GetCyclopsName _asoagame_instance))
  (Variables|Default|SetHealth 2500)
  (Variables|Default|SetValue 50000)
  (CallFunction|CheckPlayerCrouch)
  (CallFunction|Blink))

(event EventTakeDamage
  (params (DMG :type Integer))
  (bind _returnvalue (Utilities|Name|MakeLiteralName "SeenPlayer"))
  (bind _self self)
  (bind _exclamation (Variables|Default|GetExclamation))
  (bind _returnvalue_2 (AI|GetAIController _self))
  (bind _returnvalue_3 (AI|GetBlackboard _returnvalue_2))
  (CallFunction|Alert)
  (bind _output_get (Variables|Default|SetHealth (- (Variables|Default|GetHealth) DMG)))
  (if (<= _output_get 0)
    (bind _asoagame_instance (Utilities|Casting|CastToOAGameInstance (Game|GetGameInstance)))
    (Variables|/Game/Blueprints/GamemodeInstance/OAGameInstance.OAGameInstance_C|SetCredits _asoagame_instance (+ (Variables|/Game/Blueprints/GamemodeInstance/OAGameInstance.OAGameInstance_C|GetCredits _asoagame_instance) (Variables|Default|GetValue)))
    (Actor|DestroyActor)
    (else
      (bind _asoagame_instance_2 (Utilities|Casting|CastToOAGameInstance (Game|GetGameInstance)))
      (Variables|/Game/Blueprints/GamemodeInstance/OAGameInstance.OAGameInstance_C|SetCredits _asoagame_instance_2 (+ (Variables|/Game/Blueprints/GamemodeInstance/OAGameInstance.OAGameInstance_C|GetCredits _asoagame_instance_2) 100))
      (Variables|Default|SetValue (Math|Integer|Clamp(Integer) (- (Variables|Default|GetValue) 100) 0 999999))
      (Utilities|FlowControl|RetriggerableDelay 45.0)
      (AI|Components|Blackboard|SetValueasBool _returnvalue_3 _returnvalue false)
      (Variables|Default|SetChasing false)
      (Utilities|Time|ClearandInvalidateTimerbyHandle (stale Custom|Attack2 _returnvalue))
      (Utilities|FlowControl|DoOnce false) ; enters at Reset
    )))

(event EventSetName
  (bind _as_oagame_instance (Variables|Default|GetAs%20OAGame%20Instance))
  (Variables|/Game/Blueprints/GamemodeInstance/OAGameInstance.OAGameInstance_C|SetCyclopsName _as_oagame_instance (Variables|Default|GetName))
  (bind _outactors (Actor|GetAllActorsOfClass "CyclopsEnemyBP_C"))
  (for _array_element _outactors
    (Variables|/Game/Blueprints/Enemies/EnemyParentBP.EnemyParentBP_C|SetName _array_element (Variables|/Game/Blueprints/GamemodeInstance/OAGameInstance.OAGameInstance_C|GetCyclopsName _as_oagame_instance))))

(fn ConstructionScript
  (|CallParentFunction))