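; Water volume actor that changes the player character's movement to a swimming-like feel while they overlap it.
; On entry it saves the player's jump count and speed multiplier, then slows walking, sets a water gravity scale and allows long, repeated jumps.
; On exit it restores the two saved values and resets walk speed, gravity and jump hold time from hardcoded defaults.
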(event Collision|EventActorBeginOverlap
  (params (OtherActor :type Actor%20Object%20Reference))
  (bind _asplayer_character_bp (Utilities|Casting|CastToPlayerCharacterBP OtherActor))
  (Variables|Default|SetPlayerJumps (Variables|/Script/Engine.Character|GetJumpMaxCount _asplayer_character_bp))
  (Variables|Default|SetSpeed (Variables|/Game/Blueprints/Player/PlayerCharacterBP.PlayerCharacterBP_C|GetSpeedMultiplier _asplayer_character_bp))
  (bind _output_get (Variables|/Game/Blueprints/Player/PlayerCharacterBP.PlayerCharacterBP_C|SetSpeedMultiplier _asplayer_character_bp 0.7))
  (Variables|/Script/Engine.CharacterMovementComponent|SetMaxWalkSpeed (Variables|/Script/Engine.Character|GetCharacterMovement _asplayer_character_bp) (* _output_get (Variables|/Script/Engine.CharacterMovementComponent|GetMaxWalkSpeed (Variables|/Script/Engine.Character|GetCharacterMovement _asplayer_character_bp))))
  (Variables|/Script/Engine.CharacterMovementComponent|SetGravityScale (Variables|/Script/Engine.Character|GetCharacterMovement _asplayer_character_bp) 1.5)
  (Variables|/Script/Engine.Character|SetJumpMaxHoldTime _asplayer_character_bp 2e+01)
  (Variables|/Script/Engine.Character|SetJumpMaxCount _asplayer_character_bp 100))

(event Collision|EventActorEndOverlap
  (params (OtherActor :type Actor%20Object%20Reference))
  (bind _asplayer_character_bp (Utilities|Casting|CastToPlayerCharacterBP OtherActor))
  (bind _output_get (Variables|/Game/Blueprints/Player/PlayerCharacterBP.PlayerCharacterBP_C|SetSpeedMultiplier _asplayer_character_bp (Variables|Default|GetSpeed)))
  (Variables|/Script/Engine.CharacterMovementComponent|SetMaxWalkSpeed (Variables|/Script/Engine.Character|GetCharacterMovement _asplayer_character_bp) (* _output_get 3.5e+02))
  (Variables|/Script/Engine.CharacterMovementComponent|SetGravityScale (Variables|/Script/Engine.Character|GetCharacterMovement _asplayer_character_bp) 5.0)
  (Variables|/Script/Engine.Character|SetJumpMaxHoldTime _asplayer_character_bp 0.15)
  (Variables|/Script/Engine.Character|SetJumpMaxCount _asplayer_character_bp (Variables|Default|GetPlayerJumps)))

(fn ConstructionScript)