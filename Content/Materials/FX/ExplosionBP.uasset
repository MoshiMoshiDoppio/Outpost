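; ExplosionBP is a short-lived explosion effect actor built from a sphere and two rect lights.
; Each tick the sphere grows until a delay in BeginPlay sets a Shrink flag, after which it shrinks while both lights dim.
; A second delay then destroys the actor, and the scale and intensity steps are fixed per frame rather than scaled by delta time.
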(event EventBeginPlay
  (Utilities|FlowControl|Delay 0.2)
  (Variables|Default|SetShrink true)
  (Utilities|FlowControl|Delay 0.3)
  (Actor|DestroyActor))

(event EventTick
  (params (DeltaSeconds :type Float%20%28single-precision%29))
  (bind _sphere (Variables|Default|GetSphere))
  (bind _rectlight1 (Variables|Default|GetRectLight1))
  (bind _rectlight (Variables|Default|GetRectLight))
  (bind _returnvalue (Transformation|GetWorldScale _sphere))
  (if (Variables|Default|GetShrink)
    (Transformation|SetWorldScale3D _sphere (- _returnvalue "0.500000,0.500000,0.500000"))
    (Rendering|Components|Light|SetIntensity _rectlight1 (- (Variables|/Script/Engine.LightComponentBase|GetIntensity _rectlight1) 1e+04))
    (Rendering|Components|Light|SetIntensity _rectlight (- (Variables|/Script/Engine.LightComponentBase|GetIntensity _rectlight) 1e+04))
    (else
      (Transformation|SetWorldScale3D _sphere (+ _returnvalue "0.300000,0.300000,0.300000")))))

(fn ConstructionScript)